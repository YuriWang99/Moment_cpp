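; Legacy dialogue NPC Blueprint that hands its conversation off to its BP_NPC_AI controller.
; On BeginPlay it passes its DialogTree to the controller and hides a backup 3D text component.
; The Interact interface event tells the controller to start dialogue, while ExitInteract is empty.
; Every tick it rotates the backup text along the look-at direction from the player character's location to the text.
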(event `self.ReceiveBeginPlay`
  ;[0.009375 0.009375 0.009375] Put the dialog tree into the AI Controller
  (bind _asbp_npc_ai (cast `/Game/Main/NarrativeTest/AdvancedDialog/NPC/BP_NPC_AI` (`AIBlueprintHelperLibrary.GetAIController` self)))
  (set `/Game/Main/NarrativeTest/AdvancedDialog/NPC/BP_NPC_AI.DialogTree` (`self.DialogTree`) _asbp_npc_ai)
  (`SceneComponent.SetVisibility` (`self.Text3DBackup`) false false))

(event `self.ReceiveTick`
  (params (DeltaSeconds :type "Float (single-precision)"))
  (`/Game/Main/NarrativeTest/Demo/BP_FunctionLibrary_Aris.3DTextFacingCam` (`self.Text3DBackup`)))

(event `/Game/Main/NarrativeTest/AdvancedDialog/Interfaces/BPI_Interact.Interact`
  ;[0.306 0.2686 1] Interact (from Interface)
  (bind _asbp_npc_ai (cast `/Game/Main/NarrativeTest/AdvancedDialog/NPC/BP_NPC_AI` (`AIBlueprintHelperLibrary.GetAIController` self)))
  (`/Game/Main/NarrativeTest/AdvancedDialog/NPC/BP_NPC_AI.StartDialogue` _asbp_npc_ai))

(event `/Game/Main/NarrativeTest/AdvancedDialog/Interfaces/BPI_Interact.ExitInteract`)

(fn `3DTextFacingCamera`
  (params (`3DText` :type "Text3DComponent Object Reference"))
  (`SceneComponent.K2_SetWorldRotation` `3DText` (`KismetMathLibrary.FindLookAtRotation` (`self.K2_GetActorLocation` (`GameplayStatics.GetPlayerCharacter` 0)) (`SceneComponent.K2_GetComponentLocation` `3DText`)) false false))

(fn `UserConstructionScript`)