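; Audio manager actor that plays music and feedback sounds for NPC switching, interaction, mood bubbles, subtitles and winning.
; InitWwiseManager starts Wwise BGM in the Main_Room state, then binds handlers to game mode, player pawn and interaction menu dispatchers.
; Apart from the Wwise UI click, handlers mostly spawn Unreal sounds at the manager's location, often sharing one sound.
; The per-character switch is empty, and both mood branches play the same sound.
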(event `self.ReceiveBeginPlay`)

(event `InitWwiseManager`
  (bind _playerpawnref (`self.PlayerPawnRef`))
  (`AkGameplayStatics.PostEvent` "/Game/WwiseAudio/Events/Default_Work_Unit/BGM.BGM" self)
  (`AkGameplayStatics.SetState` null "BGM" "Main_Room")
  (bind _asgm_base (cast `/Game/Main/Blueprints/GameMode/GM_base` (`GameplayStatics.GetGameMode`)))
  (bind _output_get (set `self.GMRef` _asgm_base))
  (add `/Game/Main/Blueprints/GameMode/GM_base.GM_OnWinMain` _output_get (`|CreateDelegate` :!event `SFirstTaskWin`))
  (bind _asbp_character_pawn (cast `/Game/Main/Blueprints/Actors/BP_characterPawn` (`GameplayStatics.GetPlayerCharacter` 0)))
  (set `self.PlayerPawnRef` _asbp_character_pawn)
  (add `/Game/Main/Blueprints/Actors/BP_characterPawn.OnSubtitleEnd` _asbp_character_pawn (`|CreateDelegate` :!event `SubtitleEnd`))
  (add `/Game/Main/Blueprints/Actors/BP_characterPawn.OnReadNext` _asbp_character_pawn (`|CreateDelegate` :!event `SubtitleNextLine`))
  (add `/Game/Main/Blueprints/UI/BP_InteractionMenu.ShowInteraction` (`/Game/Main/Blueprints/Actors/BP_characterPawn.InteractionMenu` _playerpawnref) (`|CreateDelegate` :!event `SInteractionMenuPopup`))
  (add `/Game/Main/Blueprints/Actors/BP_characterPawn.OnReadyInteract` _playerpawnref (`|CreateDelegate` :!event `SEnterNewNPC`)))

(event `SCurrentMoodChangedHint`
  (`GameplayStatics.SpawnSoundAtLocation` "/Game/Main/Sounds/GameSounds/small-tap_Cue.small-tap_Cue" (`self.K2_GetActorLocation` self) (struct) 1.0 1.0 0.0 null null :!label _label))

(event `SFirstTaskWin`
  (goto _label))

(event `S_SwitchHoldTriggered`
  (goto _label))

(event `SObjectInteract`
  ;[1 0.9105 0.2188] Interact Sound
  (`AkGameplayStatics.PostEvent` "/Game/WwiseAudio/Events/UI_Click.UI_Click" self))

(event `SUnlockNewNPC`
  (if (`self.isFirstNPC`)
    (set `self.isFirstNPC` false)
    (else
      (`GameplayStatics.SpawnSoundAtLocation` "/Game/Main/Sounds/GameSounds/small-tap_Cue.small-tap_Cue" (`self.K2_GetActorLocation` self) (struct) 1.0 1.0 0.0 null null))))

(event `SEnterNewNPC`
  ;[0 0 0] When the player gets into another character, make some sounds to emphasize the new character's identity (Optional)
  (bind _curcharacter (`/Game/Main/Blueprints/Actors/BP_characterPawn.curCharacter` (`self.PlayerPawnRef`))
    (:`then`
      (switch `/Game/Main/Blueprints/Enum/E_NPC_names` (`/Game/Main/Blueprints/Actors/Objects/BP_NPC.name_NPC` _curcharacter)
        (:`NewEnumerator1`
          _)
        (:`NewEnumerator0`
          _)
        (:`NewEnumerator3`
          _)
        (:`NewEnumerator4`
          _)
        (:`NewEnumerator7`
          _)
        (:`NewEnumerator5`
          _))
      (`GameplayStatics.SpawnSoundAtLocation` "/Engine/EditorSounds/Notifications/CompileStart_Cue.CompileStart_Cue" (`self.K2_GetActorLocation` self) (struct) 1.0 1.0 0.0 null null))
    (:`else`)))

(event `S_ShootHeart`
  (`GameplayStatics.SpawnSoundAtLocation` "/Game/Main/Sounds/UI/SFX_Btn_Popup.SFX_Btn_Popup" (`self.K2_GetActorLocation` self) (struct) 1.0 1.0 0.0 null null :!label _label_2))

(event `SHeartExplosion`
  (goto _label_2))

(event `SubtitleNextLine`
  (goto _label_2))

(event `SubtitleEnd`
  (goto _label_2))

(event `SConfirmObject`
  (goto _label_2))

(event `SCancelConfirmObject`
  (goto _label_2))

(event `SInteractionMenuPopup`
  (params (TargetNPC :type "/Game/Main/Blueprints/Actors/Objects/BP_NPC Object Reference"))
  ;[0.02187 0.01556 0.01556] 弹出一个包含选中对象当前EMOJI 的气泡（menu）
  ;[1 0.8306 0.5596] 可以根据Emoji的内容生成不同的声音(optional)
  (switch `/Game/Main/Blueprints/Enum/E_Moods` (`/Game/Main/Blueprints/Actors/Objects/BP_NPC.CurMood` TargetNPC)
    (:`NewEnumerator4`
      (`GameplayStatics.SpawnSoundAtLocation` "/Game/Main/Sounds/SFX/Functions/SFX_UnlockNPC.SFX_UnlockNPC" (`self.K2_GetActorLocation` self) (struct) 1.0 1.0 0.0 null null :!label _label_3))
    (:`NewEnumerator0`
      (goto _label_3))
    (:`NewEnumerator1`
      (`GameplayStatics.SpawnSoundAtLocation` "/Game/Main/Sounds/SFX/Functions/SFX_UnlockNPC.SFX_UnlockNPC" (`self.K2_GetActorLocation` self) (struct) 1.0 1.0 0.0 null null :!label _label_4))
    (:`NewEnumerator2`
      (goto _label_4))
    (:`NewEnumerator3`
      (goto _label_4))))

(fn `UserConstructionScript`)