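; BP_3DTextWorldSpace is a world-space 3D text Blueprint that displays content passed to its SetContent event.
; SetContent reformats the incoming text through ReformatTextWithNewLine before applying it to the Text3D component.
; On BeginPlay it sets the Text3DCharacterTransform begin scale to zero.
; While IsFacingCamera is set, Tick calls 3DTextFacingCam on the text every frame.
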(event `self.ReceiveBeginPlay`
  (`Text3DCharacterTransform.SetScaleBegin` (`self.Text3DCharacterTransform`) (0.0 0.0 0.0)))

(event `self.ReceiveTick`
  (params (DeltaSeconds :type "Float (single-precision)"))
  (if (`self.IsFacingCamera`)
    (`/Game/Main/NarrativeTest/Demo/BP_FunctionLibrary_Aris.3DTextFacingCam` (`self.Text3D`))))

(event `SetContent`
  (params (TextToDisplay :type String))
  (bind _output (`/Game/Main/NarrativeTest/Demo/BP_FunctionLibrary_Aris.ReformatTextWithNewLine` (`KismetTextLibrary.Conv_StringToText` TextToDisplay)))
  (`Text3DComponent.SetText` (`self.Text3D`) _output))

(fn `UserConstructionScript`)