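; PC_Character is the player controller for the character pawn, caching a reference to BP_characterPawn and showing the mouse cursor on BeginPlay.
; Interface functions let other objects set and read cursor visibility.
; A debug event unlocks switching and interaction on the pawn, clears its first-time tutorial and interaction flags, and marks the first tutorial popup as done once.
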(event `self.ReceiveBeginPlay`
  (`self.getReferences`)
  (`self.Init_InputMode&Cursor`))

(event `getReferences`
  ;[0 0.4849 1] GetReference
  (bind _asbp_character_pawn (cast `/Game/Main/Blueprints/Actors/BP_characterPawn` (`GameplayStatics.GetPlayerCharacter` 0)))
  (set `self.playerCharacter_ref` _asbp_character_pawn))

(event `Init_InputMode&Cursor`
  ;[0.1483 1 0.3444] Init Input mode & cursor
  (set `self.bShowMouseCursor` true))

(event `SetDebuggingMode`
  (bind _playercharacter_ref (`self.playerCharacter_ref`))
  (bind _playercharacter_ref_2 (`self.playerCharacter_ref`))
  (set `/Game/Main/Blueprints/Actors/BP_characterPawn.SwitchAble` true _playercharacter_ref)
  (set `/Game/Main/NarrativeTest/Demo/BPW_Subtitle.FirstTimeTutorial` false (`/Game/Main/Blueprints/Actors/BP_characterPawn.SubtitleUI` _playercharacter_ref))
  (set `/Game/Main/Blueprints/Actors/BP_characterPawn.IsFirstTimeInteraction` false _playercharacter_ref)
  (`/Game/Main/Blueprints/Actors/BP_characterPawn.OnReadyInteract` _playercharacter_ref_2)
  (set `/Game/Main/Blueprints/Actors/BP_characterPawn.CanInteract` true _playercharacter_ref_2)
  (`|ExecutionSequence`
    (:`then_0`
      ;[0.0375 0.0375 0.0375] Record Tutorial 1
      (`/Engine/EditorBlueprintResources/StandardMacros.DoOnce` false
        (:`Completed`
          (set `/Game/Main/Blueprints/UI/MainMenu/WB_Tutorial.FirstTutorial` true (`/Game/Main/Blueprints/Actors/BP_characterPawn.TutPopup` (`self.playerCharacter_ref`))))))))

(event `/Game/Main/Blueprints/Interface/I_PC.setMouseCursor`
  (params (setShowMouseCursor :type Boolean))
  (set `self.bShowMouseCursor` setShowMouseCursor))

(fn `getShowMouseCursor`
  (returns (showMouseCursor :type Boolean))
  (return (`self.bShowMouseCursor`)))

(fn `UserConstructionScript`)