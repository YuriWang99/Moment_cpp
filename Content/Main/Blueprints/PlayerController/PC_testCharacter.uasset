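; Player controller for the test character that toggles the first-person widget's pause menu with the 2 key.
; On BeginPlay it caches the player character as BP_testCharacter and reaches the widget through that reference.
; Each press flips the PauseMenu flag, shows or closes the menu, and switches input mode and cursor visibility to match.
; The controller itself does not set the game's paused state.
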(event `self.ReceiveBeginPlay`
  (bind _asbp_test_character (cast `/Game/Main/Blueprints/Actors/BP_testCharacter` (`GameplayStatics.GetPlayerCharacter` 0)))
  (set `self.character_ref` _asbp_test_character))

(event `Key|Two`
  (params (Key :type "Key Structure"))
  (bind _wb_firstperson (`/Game/Main/Blueprints/Actors/BP_testCharacter.WB_FirstPerson` (`self.character_ref`)))
  (:`Pressed`
    (if (`self.PauseMenu`)
      (`/Game/Main/Blueprints/UI/WB_FirstPerson.ClosePasueMenu` _wb_firstperson)
      (set `self.PauseMenu` false)
      (`WidgetBlueprintLibrary.SetInputMode_GameOnly` self)
      (set `self.bShowMouseCursor` false)
      (else
        (`/Game/Main/Blueprints/UI/WB_FirstPerson.ShowPauseMenu` _wb_firstperson)
        (set `self.PauseMenu` true)
        (`WidgetBlueprintLibrary.SetInputMode_GameAndUIEx` self _wb_firstperson "LockOnCapture" false)
        (set `self.bShowMouseCursor` true)))))

(fn `UserConstructionScript`)