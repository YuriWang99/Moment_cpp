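; First-person test character that highlights and confirms aimed-at objects and jumps between tagged camera points.
; A per-tick camera line trace drives a crosshair state, messages the first-person widget and sets custom depth stencil values on hit meshes.
; Clicking toggles the confirmed object stored in GM_testLevel, or, on a CameraPoint actor, triggers a black screen message and moves the character to that location.
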(event `self.ReceiveBeginPlay`
  (bind _returnvalue (`|CreateWidget` "/Game/Main/Blueprints/UI/WB_FirstPerson.WB_FirstPerson_C" (`GameplayStatics.GetPlayerController` 0)))
  (bind _output_get (set `self.WB_FirstPerson` _returnvalue))
  (`UserWidget.AddToViewport` _output_get 0)
  (`WidgetBlueprintLibrary.SetInputMode_GameOnly` (`GameplayStatics.GetPlayerController` 0)))

(event `InputAxis|LookLeft/Right`
  (params (AxisValue :type "Float (single-precision)"))
  (`self.AddControllerYawInput` AxisValue))

(event `InputAxis|LookUp/Down`
  (params (AxisValue :type "Float (single-precision)"))
  (`self.AddControllerPitchInput` AxisValue))

(event `self.ReceiveTick`
  (params (DeltaSeconds :type "Float (single-precision)"))
  (bind _camera (`self.Camera`))
  (bind _returnvalue (`SceneComponent.K2_GetComponentLocation` _camera))
  (bind (_outhit _returnvalue_2) (`KismetSystemLibrary.LineTraceSingle` _returnvalue (+ _returnvalue (* (`SceneComponent.GetForwardVector` _camera) 1000.0)) "TraceTypeQuery3" false (`|MakeArray` self :!type "Actor Object Reference")))
  (if _returnvalue_2
    ;[1 1 1] ShowHitmarker
    (if (`|EnumInequality` "NewEnumerator1" (`self.CurCrosshairState`))
      _
      (elif (`self.ActorHasTag` (`.HitActor` (`GameplayStatics.BreakHitResult` _outhit)) "CameraPoint")
        (set `self.newCameraPos` (`.HitActor` (`GameplayStatics.BreakHitResult` _outhit)))
        (bind _wb_firstperson (`self.WB_FirstPerson`)
          (:`then`
            (message `/Game/Main/Blueprints/Interface/I_UI.I_ShowCameraIcon` _wb_firstperson)
            (set `self.CurCrosshairState` "NewEnumerator3"))
          (:`else`))
        (else
          (bind _output_get (set `self.HittedObj` (`.HitActor` (`GameplayStatics.BreakHitResult` _outhit))))
          (bind _asgm_test_level (cast `/Game/Main/Blueprints/GameMode/GM_testLevel` (`GameplayStatics.GetGameMode`)))
          (bind _confirmedactor (`/Game/Main/Blueprints/GameMode/GM_testLevel.ConfirmedActor` _asgm_test_level)
            (:`then`
              (if (== _confirmedactor _output_get)
                (`self.SetStencilValue` _confirmedactor 2)
                (bind _wb_firstperson_2 (`self.WB_FirstPerson`)
                  (:`then`
                    (message `/Game/Main/Blueprints/Interface/I_UI.I_ShowHitConfirm` _wb_firstperson_2)
                    (set `self.CurCrosshairState` "NewEnumerator2"))
                  (:`else`))
                (else
                  (`self.SetStencilValue` _output_get 1 :!label _label)
                  (bind _wb_firstperson_3 (`self.WB_FirstPerson`)
                    (:`then`
                      (message `/Game/Main/Blueprints/Interface/I_UI.I_ShowHitMarker` _wb_firstperson_3)
                      (set `self.CurCrosshairState` "NewEnumerator0"))
                    (:`else`)))))
            (:`else`
              (goto _label))))))
    (else
      ;[1 1 1] Close Hitmarker
      (if (`|EnumEquality` (`self.CurCrosshairState`) "NewEnumerator0")
        (`self.SetStencilValue` (`self.HittedObj`))
        (bind _wb_firstperson_4 (`self.WB_FirstPerson` :!label _label_2)
          (:`then`
            (message `/Game/Main/Blueprints/Interface/I_UI.I_CloseHitMarker` _wb_firstperson_4)
            (set `self.HittedObj` null :!label _label_3)
            (set `self.CurCrosshairState` "NewEnumerator1"))
          (:`else`))
        (elif (`|EnumEquality` (`self.CurCrosshairState`) "NewEnumerator2")
          (goto _label_2)
          (elif (`|EnumEquality` (`self.CurCrosshairState`) "NewEnumerator3")
            (bind _wb_firstperson_5 (`self.WB_FirstPerson`)
              (:`then`
                (message `/Game/Main/Blueprints/Interface/I_UI.I_CloseCameraIcon` _wb_firstperson_5)
                (goto _label_3))
              (:`else`))))))))

(event `SetStencilValue`
  (params (Actor :type "Actor Object Reference") (StencilValue :type Integer))
  (`/Engine/EditorBlueprintResources/StandardMacros.IsValid` Actor
    (:`Is Valid`
      (`PrimitiveComponent.SetCustomDepthStencilValue` (`self.GetComponentByClass` Actor "/Script/Engine.StaticMeshComponent") StencilValue))))

(event `InputAction|Mouse_0`
  (params (Key :type "Key Structure"))
  ;[1 1 1] Show Hit Confirm
  (:`Pressed`
    (if (`|EnumEquality` "NewEnumerator0" (`self.CurCrosshairState`))
      (bind _wb_firstperson (`self.WB_FirstPerson`)
        (:`then`
          (message `/Game/Main/Blueprints/Interface/I_UI.I_ShowHitConfirm` _wb_firstperson)
          (set `self.CurCrosshairState` "NewEnumerator2")
          (bind _asgm_test_level (cast `/Game/Main/Blueprints/GameMode/GM_testLevel` (`GameplayStatics.GetGameMode`)))
          (bind _confirmedactor (`/Game/Main/Blueprints/GameMode/GM_testLevel.ConfirmedActor` _asgm_test_level)
            (:`then`
              (`self.SetStencilValue` _confirmedactor))
            (:`else`
              _))
          (bind _hittedobj (`self.HittedObj`)
            (:`then`
              (bind _output_get (set `/Game/Main/Blueprints/GameMode/GM_testLevel.ConfirmedActor` _hittedobj _asgm_test_level))
              (`self.SetStencilValue` _output_get 2))
            (:`else`)))
        (:`else`))
      (else
        ;[1 1 1] Close Hit Confirm
        (if (`|EnumEquality` "NewEnumerator2" (`self.CurCrosshairState`))
          (bind _wb_firstperson_2 (`self.WB_FirstPerson`)
            (:`then`
              (message `/Game/Main/Blueprints/Interface/I_UI.I_CloseHitConfirm` _wb_firstperson_2)
              (set `self.CurCrosshairState` "NewEnumerator0")
              (bind _asgm_test_level_2 (cast `/Game/Main/Blueprints/GameMode/GM_testLevel` (`GameplayStatics.GetGameMode`)))
              (bind _confirmedactor_2 (`/Game/Main/Blueprints/GameMode/GM_testLevel.ConfirmedActor` _asgm_test_level_2)
                (:`then`
                  (`self.SetStencilValue` _confirmedactor_2 1)
                  (set `/Game/Main/Blueprints/GameMode/GM_testLevel.ConfirmedActor` null _asgm_test_level_2))
                (:`else`)))
            (:`else`))
          (elif (`|EnumEquality` "NewEnumerator3" (`self.CurCrosshairState`))
            (bind _wb_firstperson_3 (`self.WB_FirstPerson`)
              (:`then`
                (message `/Game/Main/Blueprints/Interface/I_UI.I_ShowBlackScreen` _wb_firstperson_3)
                (bind _newcamerapos (`self.newCameraPos`)
                  (:`then`
                    (`self.SwithCameraPos` _newcamerapos)
                    (set `self.CurCrosshairState` "NewEnumerator1"))
                  (:`else`)))
              (:`else`))))))))

(event `InputAction|Mouse_1`
  (params (Key :type "Key Structure")))

(event `SwithCameraPos`
  (params (newActorPos :type "Actor Object Reference"))
  (bind _returnvalue_location (`KismetMathLibrary.BreakTransform` (`self.GetTransform` newActorPos)))
  (`self.K2_SetActorRelativeLocation` _returnvalue_location))

(fn `UserConstructionScript`)