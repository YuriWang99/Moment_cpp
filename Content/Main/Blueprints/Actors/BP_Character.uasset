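; BP_Character is a character actor Blueprint that detects which interactable object sits under the mouse cursor.
; BeginPlay caches GM_base and GI_Player references and resets the cursor to default, while the level init event is an empty stub.
; Every Tick it traces under the cursor, stores actors tagged InteractableObject in HittedObj, clears it otherwise, and prints the name for debugging.
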(event `self.ReceiveBeginPlay`
  (`|ExecutionSequence`
    (:`then_0`
      (`self.init_references`)
      (`self.Init_UI`)
      (`self.Init_Level`))))

(event `Init_Level`)

(event `Init_UI`
  ;[0.2282 1 0.2508] init UI
  (`self.ResetCursorIcon`))

(event `init_references`
  ;[0 0.4849 1] get references
  (`|ExecutionSequence`
    (:`then_0`
      (bind _asgm_base (cast `/Game/Main/Blueprints/GameMode/GM_base` (`GameplayStatics.GetGameMode`)))
      (set `self.GM_ref` _asgm_base))
    (:`then_1`
      (bind _asgi_player (cast `/Game/Main/Blueprints/GameInstance/GI_Player` (`GameplayStatics.GetGameInstance`)))
      (set `self.GI_ref` _asgi_player))))

(event `self.ReceiveTick`
  (params (DeltaSeconds :type "Float (single-precision)"))
  (`self.mouseHit`)
  (`KismetSystemLibrary.PrintString` (`KismetSystemLibrary.GetObjectName` (`self.HittedObj`))))

(event `mouseHit`
  (bind (_hitresult _returnvalue) (`PlayerController.GetHitResultUnderCursorByChannel` (`GameplayStatics.GetPlayerController` 0) "TraceTypeQuery3" false))
  (if _returnvalue
    (`self.SetHittedObj` (`.HitActor` (`GameplayStatics.BreakHitResult` _hitresult)) "InteractableObject")
    (else
      (set `self.HittedObj` null))))

(fn `ResetCursorIcon`
  (set `PlayerController.CurrentMouseCursor` "Default" (`GameplayStatics.GetPlayerController` 0)))

(fn `SetHittedObj`
  (params (Actor :type "Actor Object Reference") (Tag :type Name))
  (if (`self.ActorHasTag` Actor Tag)
    (if (!= (`local.Actor`) (`self.HittedObj`))
      (set `self.HittedObj` (`local.Actor`)))
    (else
      (set `self.HittedObj` null))))

(fn `UserConstructionScript`)