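; Child character Blueprint that lets the player interact with objects, such as NPCs, implementing BPI_Interact.
; Each Tick, InteractionCheck line traces forward from the camera and shows or hides a prompt on the HUD fetched from GM_testLevel.
; IA_Interact or the E key repeats the trace, prints a debug string and calls InteractMessage on the returned actor.
; PointerHover runs on Tick but is an empty stub for 3D UI interaction.
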(event `self.ReceiveBeginPlay`
  (`parent.ReceiveBeginPlay`)
  ;[1 0.1208 0.1786] Dialogue HUD Setup
  (bind _asgm_test_level (cast `/Game/Main/Blueprints/GameMode/GM_testLevel` (`GameplayStatics.GetGameMode`)))
  (set `self.PlayerHUD` (`/Game/Main/Blueprints/GameMode/GM_testLevel.HUD` _asgm_test_level)))

(event `self.ReceiveTick`
  (params (DeltaSeconds :type "Float (single-precision)"))
  ;[1 0.1216 0.1804] Interact With NPC and Show Dialogue
  (`parent.ReceiveTick` DeltaSeconds)
  (`self.InteractionCheck`) ; Display NPC Interaction Message
  (`self.PointerHover`))

(event `EnhancedInput|/Game/FirstPerson/Input/Actions/IA_Interact`
  (params (ActionValue :type Boolean) (ElapsedSeconds :type "Float (double-precision)") (TriggeredSeconds :type "Float (double-precision)") (InputAction :type "InputAction Object Reference" :default "/Game/FirstPerson/Input/Actions/IA_Interact.IA_Interact"))
  ;[1 0.1216 0.1804] Interact With NPC and Show Dialogue
  (:`Triggered`
    (bind _actor (`self.InteractionCheck` :!label _label))
    (`KismetSystemLibrary.PrintString` "Interaction start" true true (struct :`R` 1.0 :`G` 0.251122 :`B` 0.16141 :`A` 1.0))
    (message `/Game/Main/NarrativeTest/AdvancedDialog/Interfaces/BPI_Interact.Interact` _actor)))

(event `Key|E`
  (params (Key :type "Key Structure"))
  ;[1 0.1216 0.1804] Interact With NPC and Show Dialogue
  (:`Pressed`
    (goto _label)))

(event `PointerHover`)

(fn `InteractionCheck`
  (returns (Actor :type "Actor Object Reference"))
  (locals (InteractActor :type "Actor Object Reference"))
  (bind _camera (`self.Camera`))
  (bind _playerhud (`self.PlayerHUD`))
  (bind _returnvalue (`SceneComponent.K2_GetComponentLocation` _camera))
  (bind _outhit (`KismetSystemLibrary.LineTraceSingle` _returnvalue (+ _returnvalue (* (`SceneComponent.GetForwardVector` _camera) 2000.0)) "TraceTypeQuery3" false (`|MakeArray` self :!type "Actor Object Reference")))
  (if (`GameplayStatics.BreakHitResult` _outhit)
    (if (`KismetSystemLibrary.DoesImplementInterface` (`.HitActor` (`GameplayStatics.BreakHitResult` _outhit)) "/Game/Main/NarrativeTest/AdvancedDialog/Interfaces/BPI_Interact.BPI_Interact_C")
      (bind _output_get (set `local.InteractActor` (`.HitActor` (`GameplayStatics.BreakHitResult` _outhit))))
      (`/Game/Main/NarrativeTest/AdvancedDialog/UserInterface/BPW_HUD.DisplayMessage` _playerhud true _output_get)
      (return (`local.InteractActor`))
      (else
        _)))
  (`/Game/Main/NarrativeTest/AdvancedDialog/UserInterface/BPW_HUD.DisplayMessage` _playerhud false null)
  (return null))

(fn `UserConstructionScript`
  (`parent.UserConstructionScript`))