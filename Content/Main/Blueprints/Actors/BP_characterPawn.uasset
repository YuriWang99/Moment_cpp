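; Player pawn for a point-and-click game in which the player switches viewpoint between NPC characters and confirms an object for each.
; Tick traces under the cursor and highlights hovered interactable objects through custom-depth stencil values.
; Left-click on an NPC swaps its collision response and moves the camera by location, then rotation timelines.
; Right-click toggles the current character's confirmed object, restored on switch; the win check is a stub.
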(event `self.ReceiveBeginPlay`
  (`|ExecutionSequence`
    (:`then_0`
      (`self.init_references`)
      (`self.Init_UI`))))

(event `Init_character`
  ;[1 0.8883 0.09038] Init_character
  (for _array_element (`self.characterList`)
    (if (== (`/Game/Main/Blueprints/Actors/Objects/BP_NPC.PlayerView` _array_element) (`self.startView`))
      (set `self.curPlayerView` (`self.startView`))
      (bind _output_get (set `self.curCharacter` _array_element))
      (`self.SetCollisionResponseToChannel` _output_get)
      (break))))

(event `Init_UI`
  ;[0.2282 1 0.2508] init UI
  (`self.ResetCursorIcon`))

(event `Init_Camera`)

(event `init_references`
  ;[0 0.4849 1] get references
  (`|ExecutionSequence`
    (:`then_0`
      (bind _asgm_base (cast `/Game/Main/Blueprints/GameMode/GM_base` (`GameplayStatics.GetGameMode`)))
      (set `self.GM_ref` _asgm_base))
    (:`then_1`
      (bind _asgi_player (cast `/Game/Main/Blueprints/GameInstance/GI_Player` (`GameplayStatics.GetGameInstance`)))
      (set `self.GI_ref` _asgi_player))
    (:`then_2`
      (bind _aspc_character (cast `/Game/Main/Blueprints/PlayerController/PC_Character` (`GameplayStatics.GetPlayerController` 0)))
      (set `self.PC_Character_ref` _aspc_character))
    (:`then_3`
      ;;[1 1 1] Store the reference to the Interaction Menu
      (bind _returnvalue (`GameplayStatics.GetActorOfClass` "/Game/Main/Blueprints/UI/BP_InteractionMenu.BP_InteractionMenu_C"))
      (set `self.InteractionMenu` _returnvalue)
      (`self.InitNPCUI`))))

(event `InitNPCUI`
  ;[0.7765 1 0.3922] NPC Mood UI
  (bind _returnvalue (`|CreateWidget` "/Game/Main/Blueprints/UI/BPW_MoodProfile.BPW_MoodProfile_C" (`GameplayStatics.GetPlayerController` 0)))
  (bind _output_get (set `self.NPCUI` _returnvalue))
  (`UserWidget.AddToViewport` _output_get 0)
  (`/Game/Main/Blueprints/UI/BPW_MoodProfile.InitShowMoodUI` _output_get))

(event `LoadNPCList`)

(event `self.ReceiveTick`
  (params (DeltaSeconds :type "Float (single-precision)"))
  (`self.mouseHit`))

(event `mouseHit`
  (bind _returnvalue (`GameplayStatics.GetPlayerController` 0))
  (bind (_hitresult _returnvalue_2) (`PlayerController.GetHitResultUnderCursorByChannel` _returnvalue "TraceTypeQuery3" false))
  ;[0.1483 1 0.3444] control & interaction
  (bind _showmousecursor (message `/Game/Main/Blueprints/Interface/I_PC.getShowMouseCursor` _returnvalue))
  (if _showmousecursor
    (`self.Set Hitted Obj` (`.HitActor` (`GameplayStatics.BreakHitResult` _hitresult)) "InteractableObject" _returnvalue_2)
    (`self.ResetCursorIcon`)
    (`self.Init_curConfrimedObj` (`self.curCharacter`))
    ;;[0.6937 0.4671 1] Control Open / Close Interaction Menu
    (bind _hittedobj (`self.HittedObj`)
      (:`then`)
      (:`else`
        (if (`.ReturnValue` (`PlayerController.GetHitResultUnderCursorByChannel` _returnvalue "TraceTypeQuery4" false))
          _)))))

(event `InputAction|Mouse_0`
  (params (Key :type "Key Structure"))
  ;[0.1483 1 0.3444] control & interaction
  (:`Released`
    (bind _hittedobj (`self.HittedObj`)
      (:`then`
        (if (`self.ActorHasTag` _hittedobj "NPC")
          (`KismetSystemLibrary.PrintString` "弹出UI")
          (bind _asbp_npc (cast `/Game/Main/Blueprints/Actors/Objects/BP_NPC` (`self.HittedObj`)))
          (`self.SwitchCharacter` _asbp_npc)
          (else
            (`KismetSystemLibrary.PrintString` "Read"))))
      (:`else`))))

(event `InputAction|Mouse_1`
  (params (Key :type "Key Structure"))
  ;[0.1483 1 0.3444] control & interaction
  (:`Released`
    (`self.ConfirmBehavior`)))

(event `ConfirmBehavior`
  ;[0.1483 1 0.3444] control & interaction
  (bind _hittedobj (`self.HittedObj`)
    (:`then`
      (if (!= _hittedobj (`self.curConfirmedObj`))
        (`self.ConfirmedObject` (`self.HittedObj`))
        (else
          (`self.cancelConfirmObject`))))
    (:`else`
      (`self.ConfirmedObject` (`self.HittedObj`)))))

(event `SwitchCharacter`
  (params (NPC :type "/Game/Main/Blueprints/Actors/Objects/BP_NPC Object Reference"))
  ;[1 0.7401 0.03929] Switch Character
  (`|ExecutionSequence`
    (:`then_0`
      (`self.Init_characterValue` NPC))
    (:`then_1`
      (`self.ClearCurConfirmedObject`)
      (`self.ResetCurCharacter` NPC))
    (:`then_2`
      (message `/Game/Main/Blueprints/Interface/I_PC.setMouseCursor` (`GameplayStatics.GetPlayerController` 0) false)
      (`self.SetNewView` null)
      (message `/Game/Main/Blueprints/Interface/I_PC.setMouseCursor` (`GameplayStatics.GetPlayerController` 0) true))))

(event `SetNewView`
  (params (newNPC :type "/Game/Main/Blueprints/Actors/Objects/BP_NPC Object Reference"))
  ;[0.4485 1 0.3662] Lerp the camera to the target
  (bind (_direction _duration) (`Timeline|LerpCharacterLocation` :!via `PlayFromStart`)
    (:`Update`
      (`self.K2_SetActorLocation` (`KismetMathLibrary.VLerp` (`self.curCameraLocation`) (`self.newCameraLocation`) _duration)))
    (:`Finished`
      (bind (_direction_2 _duration_2) (`Timeline|LerpCharacterRotation` :!via `PlayFromStart`)
        (:`Update`
          (`Controller.SetControlRotation` (`GameplayStatics.GetPlayerController` 0) (`KismetMathLibrary.RLerp` (`self.curCameraRotation`) (`self.newCameraRotation`) _duration_2)))))))

(fn `cancelConfirmObject`
  (set `/Game/Main/Blueprints/Actors/Objects/BP_NPC.ConfirmedObj` null (`self.curCharacter`))
  (`self.ClearCurConfirmedObject`))

(fn `checkWin`)

(fn `ClearCurConfirmedObject`
  (bind _curconfirmedobj (`self.curConfirmedObj`)
    (:`then`
      (`self.SetStencilValue` _curconfirmedobj)
      (set `self.curConfirmedObj` null))
    (:`else`)))

(fn `ConfirmedObject`
  (params (HittedObj :type "/Game/Main/Blueprints/Actors/Objects/BP_ObjectBase Object Reference"))
  (`self.ClearCurConfirmedObject`)
  (bind _output_get (set `self.curConfirmedObj` HittedObj))
  (bind _output_get_2 (set `/Game/Main/Blueprints/Actors/Objects/BP_NPC.ConfirmedObj` _output_get (`self.curCharacter`)))
  (`self.SetStencilValue` _output_get_2 2)
  (`self.checkWin`))

(fn `Init_characterValue`
  (params (newNPC :type "/Game/Main/Blueprints/Actors/Objects/BP_NPC Object Reference"))
  (bind _curcharacter (`self.curCharacter`))
  (bind _returnvalue (`SceneComponent.K2_GetComponentRotation` (`Actor.RootComponent` newNPC)))
  (set `self.newCameraRotation` _returnvalue) ; currently using the CharacterPawn Rotation
  (set `self.newCameraLocation` (+ (`SceneComponent.K2_GetComponentLocation` (`/Game/Main/Blueprints/Actors/Objects/BP_NPC.CameraPoint` newNPC)) (* (`KismetMathLibrary.GetForwardVector` _returnvalue) 10.0)))
  (set `self.curCameraLocation` (`SceneComponent.K2_GetComponentLocation` (`/Game/Main/Blueprints/Actors/Objects/BP_NPC.CameraPoint` _curcharacter)))
  (set `self.curCameraRotation` (`SceneComponent.K2_GetComponentRotation` (`/Game/Main/Blueprints/Actors/Objects/BP_ObjectBase.DefaultSceneRoot` _curcharacter))))

(fn `Init_curConfrimedObj`
  (params (NPC :type "/Game/Main/Blueprints/Actors/Objects/BP_NPC Object Reference"))
  (bind _confirmedobj (`/Game/Main/Blueprints/Actors/Objects/BP_NPC.ConfirmedObj` NPC)
    (:`then`
      (bind _output_get (set `self.curConfirmedObj` _confirmedobj))
      (`self.SetStencilValue` _output_get 2))
    (:`else`
      (set `self.curConfirmedObj` null))))

(fn `ResetCurCharacter`
  (params (newNPC :type "/Game/Main/Blueprints/Actors/Objects/BP_NPC Object Reference"))
  (locals (NewNPCLocal :type "/Game/Main/Blueprints/Actors/Objects/BP_NPC Object Reference"))
  (bind _curcharacter (`self.curCharacter`))
  (set `local.NewNPCLocal` newNPC)
  (message `/Game/Main/Blueprints/Interface/I_PC.setMouseCursor` (`GameplayStatics.GetPlayerController` 0) false)
  (for _array_element (`self.characterList`)
    (if (== _array_element (`local.NewNPCLocal`))
      (`self.SetCollisionResponseToChannel` (`self.curCharacter`) "ECR_Block")
      (bind _output_get (set `self.curCharacter` (`local.NewNPCLocal`)))
      (`self.SetCollisionResponseToChannel` _output_get "ECR_Overlap")
      (set `self.curPlayerView` (`/Game/Main/Blueprints/Actors/Objects/BP_NPC.PlayerView` _curcharacter))
      (`self.Init_curConfrimedObj` _curcharacter)
      (break)))
  (message `/Game/Main/Blueprints/Interface/I_PC.setMouseCursor` (`GameplayStatics.GetPlayerController` 0) true))

(fn `ResetCursorIcon`
  (set `PlayerController.CurrentMouseCursor` "Default" (`GameplayStatics.GetPlayerController` 0)))

(fn `ResetHittedObj`
  ;[0.1483 1 0.3444] un highlight the current hitted object
  (bind _hittedobj (`self.HittedObj`)
    (:`then`
      (`self.SetStencilValue` _hittedobj)
      (set `self.HittedObj` null))
    (:`else`)))

(fn `Set Hitted Obj`
  (params (Actor :type "Actor Object Reference") (Tag :type Name) (Hitted :type Boolean))
  (locals (ObjectBase :type "/Game/Main/Blueprints/Actors/Objects/BP_ObjectBase Object Reference"))
  (if Hitted
    (bind _asbp_object_base (cast `/Game/Main/Blueprints/Actors/Objects/BP_ObjectBase` Actor)
      (:`then`
        (bind _output_get (set `local.ObjectBase` _asbp_object_base))
        (if (`self.ActorHasTag` _output_get Tag)
          (if (!= (`local.ObjectBase`) (`self.HittedObj`))
            (bind _output_get_2 (set `self.HittedObj` (`local.ObjectBase`)))
            (`self.SetStencilValue` _output_get_2 1)
            ;[0.6911 0.5627 1] Track the hitted obj (before it is set null)
            (bind _hittedobj (`self.HittedObj`)
              (:`then`
                (set `self.HittedObj_previous` _hittedobj))
              (:`else`)))
          (else
            (`self.ResetHittedObj`))))
      (:`CastFailed`
        (`self.ResetHittedObj`)))
    (else
      (`self.ResetHittedObj`))))

(fn `SetCollisionResponseToChannel`
  (params (NPC :type "/Game/Main/Blueprints/Actors/Objects/BP_NPC Object Reference") (CollisionChannel :type "ECollisionResponse Enum" :default "ECR_Ignore"))
  (`PrimitiveComponent.SetCollisionResponseToChannel` (`/Game/Main/Blueprints/Actors/Objects/BP_ObjectBase.MainMesh` NPC) "ECC_GameTraceChannel1" CollisionChannel)
  (`PrimitiveComponent.SetCollisionResponseToChannel` (`/Game/Main/Blueprints/Actors/Objects/BP_NPC.CameraPoint` NPC) "ECC_GameTraceChannel1" CollisionChannel)
  (`KismetSystemLibrary.PrintString` "Hello"))

(fn `SetStencilValue`
  (params (ObjectBasse :type "/Game/Main/Blueprints/Actors/Objects/BP_ObjectBase Object Reference") (StencilValue :type Integer))
  (bind _returnvalue (`self.GetComponentsByTag` ObjectBasse "/Script/Engine.SkeletalMeshComponent" "Mesh"))
  (bind _returnvalue_2 (`self.GetComponentsByTag` ObjectBasse "/Script/Engine.StaticMeshComponent" "Mesh"))
  (if (`KismetArrayLibrary.Array_IsNotEmpty` _returnvalue_2)
    (`PrimitiveComponent.SetCustomDepthStencilValue` (`|GetArrayItem` _returnvalue_2) StencilValue)
    (elif (`KismetArrayLibrary.Array_IsNotEmpty` _returnvalue)
      (`PrimitiveComponent.SetCustomDepthStencilValue` (`|GetArrayItem` _returnvalue) StencilValue))))

(fn `UserConstructionScript`)