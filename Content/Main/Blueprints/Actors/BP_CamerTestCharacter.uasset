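; Test character for trying out a cursor-driven, angle-limited camera view.
; On BeginPlay it adds the WB_CursorTest widget, shows the mouse cursor and clamps the camera manager's yaw and pitch using per-PlayerView limits, with yaw relative to actor rotation.
; LookUp runs a timeline that sets control pitch from 0 to 20 and prints it.
; Other look events and axis inputs are empty, with older controller-input logic left disconnected.
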(event `InputAxis|LookLeft/Right`
  (params (AxisValue :type "Float (single-precision)")))

(event `InputAxis|LookUp/Down`
  (params (AxisValue :type "Float (single-precision)")))

(event `self.ReceiveBeginPlay`
  (bind _returnvalue (`GameplayStatics.GetPlayerController` 0))
  (bind _returnvalue_2 (`|CreateWidget` "/Game/Main/Blueprints/UI/WB_CursorTest.WB_CursorTest_C" _returnvalue))
  (`UserWidget.AddToViewport` _returnvalue_2 0)
  (set `PlayerController.bShowMouseCursor` true _returnvalue)
  (`self.InitCamera`))

(event `LookUp`
  (bind (_direction _newtrack_0) (`Timeline|LerpTest` :!via `PlayFromStart`)
    (:`Update`
      (bind _returnvalue (`KismetMathLibrary.Lerp` 0.0 20.0 _newtrack_0))
      (`KismetSystemLibrary.PrintString` (`KismetStringLibrary.Conv_DoubleToString` _returnvalue))
      (`Controller.SetControlRotation` (`GameplayStatics.GetPlayerController` 0) (`KismetMathLibrary.MakeRotator` 0.0 _returnvalue)))))

(event `LookDown`)

(event `LookLeft`)

(event `LookRight`)

(fn `InitCamera`
  (bind _returnvalue (`GameplayStatics.GetPlayerCameraManager` 0))
  (bind _playerview (`self.playerView`))
  (bind (_returnvalue_roll _returnvalue_pitch _returnvalue_yaw) (`KismetMathLibrary.BreakRotator` (`self.K2_GetActorRotation` self)))
  (set `PlayerCameraManager.ViewYawMax` (+ _returnvalue_yaw (`|GetArrayItem` (`self.YawMax`) _playerview)) _returnvalue)
  (set `PlayerCameraManager.ViewYawMin` (+ _returnvalue_yaw (`|GetArrayItem` (`self.YawMin`) _playerview)) _returnvalue)
  (set `PlayerCameraManager.ViewPitchMax` (`|GetArrayItem` (`self.PitchMax`) _playerview) _returnvalue)
  (set `PlayerCameraManager.ViewPitchMin` (`|GetArrayItem` (`self.PitchMin`) _playerview) _returnvalue))

(fn `UserConstructionScript`)