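; BP_PPSManager switches the post-process look to match the current NPC character.
; It binds to player pawn events on BeginPlay, and SetNPCPPS resets to default cel shading, then applies per-NPC looks.
; These include mood-driven grayscale for Boring Worker, no cel shading for Boss, and underwater for Turtle.
; Timelines drive MPC_PPS parameters for desaturation and vignette, while underwater swaps a tagged volume's settings and toggles a decal.
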(event `GrayscaleToColorful`
  (params (IsGradient :type Boolean))
  (if (`self.IsGray`)
    (if IsGradient
      ;[0.2215 0.5778 1] Greyscale->Colorful
      (switch `/Game/Main/Blueprints/Enum/E_NPC_names` (`/Game/Main/Blueprints/Actors/Objects/BP_NPC.name_NPC` (`/Game/Main/Blueprints/Actors/BP_characterPawn.PreviousCharacter` (`self.PlayerRef`)))
        (:`NewEnumerator5`
          (set `self.IsGray` false)
          (bind (_direction _desaturation) (`Timeline|Timeline_0` :!via `ReverseFromEnd`)
            (:`Update`
              (`KismetMaterialLibrary.SetScalarParameterValue` "/Game/MPC_PPS.MPC_PPS" "CelShadingDesatuation" _desaturation)))))
      (else
        (set `self.IsGray` false)
        (bind (_direction_2 _desaturation_2) (`Timeline|RapidChange` :!via `PlayFromStart`)
          (:`Update`
            (`KismetMaterialLibrary.SetScalarParameterValue` "/Game/MPC_PPS.MPC_PPS" "CelShadingDesatuation" _desaturation_2)))))))

(event `BoringSad`
  (bind _curcharacter (`/Game/Main/Blueprints/Actors/BP_characterPawn.curCharacter` (`self.PlayerRef`)))
  (if (`|EnumEquality` (`/Game/Main/Blueprints/Actors/Objects/BP_NPC.name_NPC` _curcharacter) "NewEnumerator5")
    (`self.SetNPCPPS` _curcharacter)))

(event `self.ReceiveBeginPlay`
  (bind _playerref (`self.PlayerRef`))
  (bind _asbp_character_pawn (cast `/Game/Main/Blueprints/Actors/BP_characterPawn` (`GameplayStatics.GetPlayerCharacter` 0)))
  (set `self.PlayerRef` _asbp_character_pawn)
  (add `/Game/Main/Blueprints/Actors/BP_characterPawn.OnConfirmTriggered` _playerref (`|CreateDelegate` :!event `ConfirmChangePPS`))
  (add `/Game/Main/Blueprints/Actors/BP_characterPawn.OnSubtitleStart` _playerref (`|CreateDelegate` :!event `TurnOnVignette`))
  (add `/Game/Main/Blueprints/Actors/BP_characterPawn.OnSubtitleEnd` _playerref (`|CreateDelegate` :!event `TurnOffVignette`))
  (add `/Game/Main/Blueprints/Actors/BP_characterPawn.OnFinishSwitchView` _playerref (`|CreateDelegate` :!event `SetNPCPPS`))
  (add `/Game/Main/Blueprints/Actors/BP_characterPawn.OnLoveTriangleCanceled` _playerref (`|CreateDelegate` :!event `BoringSad`))
  (add `/Game/Main/Blueprints/Actors/BP_characterPawn.OnLoveTriangleTriggered` _playerref (`|CreateDelegate` :!event `BoringSad`)))

(event `SetNPCPPS`
  (params (NewNPC :type "/Game/Main/Blueprints/Actors/Objects/BP_NPC Object Reference"))
  (bind _playerref (`self.PlayerRef`))
  (`KismetSystemLibrary.PrintString` "Set PPS" true true (struct :`R` 0.551856 :`G` 0.02411 :`B` 1.0 :`A` 1.0) 3.0)
  (switch `/Game/Main/Blueprints/Enum/E_NPC_names` (`/Game/Main/Blueprints/Actors/Objects/BP_NPC.name_NPC` NewNPC)
    (:`NewEnumerator1`
      (`self.ResetDefaultPPS` :!label _label)
      (`self.GrayscaleToColorful` false))
    (:`NewEnumerator0`
      (goto _label))
    (:`NewEnumerator4`
      (goto _label))
    (:`NewEnumerator7`
      (goto _label))
    (:`NewEnumerator5`
      (`self.ResetDefaultPPS`)
      (if (`|EnumEquality` (`/Game/Main/Blueprints/Actors/Objects/BP_NPC.CurMood` NewNPC) "NewEnumerator0")
        (`self.GrayscaleToColorful` true)
        (`KismetSystemLibrary.PrintString` "Happy Boring" true true (struct :`G` 1.0 :`B` 0.476364 :`A` 1.0))
        (set `Widget.Visibility` "Hidden" (`/Game/Main/Blueprints/Actors/BP_characterPawn.BPWSleepy` (`self.PlayerRef`)))
        (else
          (`self.ColorfulToGrayscale`)
          (set `Widget.Visibility` "Visible" (`/Game/Main/Blueprints/Actors/BP_characterPawn.BPWSleepy` _playerref))
          (`/Engine/EditorBlueprintResources/StandardMacros.DoOnce` false
            (:`Completed`
              (`/Game/Main/NarrativeTest/Demo/BPW_Subtitle.ShowAwakeTut` (`/Game/Main/Blueprints/Actors/BP_characterPawn.SubtitleUI` _playerref)))))))
    (:`NewEnumerator8`
      (`self.ResetDefaultPPS`)
      (`self.DisableCelShading`)
      (`/Game/Main/Blueprints/Actors/BP_characterPawn.DoFPPSStartup` (`self.PlayerRef`)))
    (:`NewEnumerator9`
      (goto _label))
    (:`NewEnumerator10`
      (`self.TurnOnUnderWater`))
    (:`NewEnumerator3`
      (`self.ResetDefaultPPS` :!label _label_2))
    (:`NewEnumerator11`
      (goto _label_2))))

(event `UnbindVignette`
  (bind _playerref (`self.PlayerRef`))
  (remove `/Game/Main/Blueprints/Actors/BP_characterPawn.OnSubtitleStart` _playerref (`|CreateDelegate` :!event `TurnOnVignette`))
  (remove `/Game/Main/Blueprints/Actors/BP_characterPawn.OnSubtitleEnd` _playerref (`|CreateDelegate` :!event `TurnOffVignette`)))

(event `ColorfulToGrayscale`
  (if (not (`self.IsGray`))
    ;[0.05104 0.05104 0.05104] Colorful->Greyscale
    (set `self.IsGray` true)
    (bind (_direction _desaturation) (`Timeline|Timeline` :!via `PlayFromStart`)
      (:`Update`
        (`KismetMaterialLibrary.SetScalarParameterValue` "/Game/MPC_PPS.MPC_PPS" "CelShadingDesatuation" _desaturation)))))

(event `TurnOnUnderWater`
  (bind _outactors (`GameplayStatics.GetAllActorsOfClassWithTag` "/Script/Engine.PostProcessVolume" "SpecialPPV"))
  (set `PostProcessVolume.Settings` (make `PostProcessSettings` :`WeightedBlendables` (`self.UnderWaterPPS`)) (`|GetArrayItem` _outactors))
  (bind _returnvalue (`GameplayStatics.GetActorOfClass` "/Script/Engine.DecalActor"))
  (`SceneComponent.SetVisibility` (`DecalActor.Decal` _returnvalue) true false))

(event `DisableCelShading`
  (`KismetMaterialLibrary.SetScalarParameterValue` "/Game/MPC_PPS.MPC_PPS" "CelShadingIntensity"))

(event `EnableCelShading`
  (`KismetMaterialLibrary.SetScalarParameterValue` "/Game/MPC_PPS.MPC_PPS" "CelShadingIntensity" 1.0))

(event `TurnOffUnderWater`
  (bind _returnvalue (`GameplayStatics.GetActorOfClass` "/Script/Engine.DecalActor"))
  (`SceneComponent.SetVisibility` (`DecalActor.Decal` _returnvalue) false false)
  (bind _outactors (`GameplayStatics.GetAllActorsOfClassWithTag` "/Script/Engine.PostProcessVolume" "SpecialPPV"))
  (set `PostProcessVolume.Settings` (make `PostProcessSettings`) (`|GetArrayItem` _outactors)))

(event `ConfirmChangePPS`
  (`self.SetNPCPPS` (`/Game/Main/Blueprints/Actors/BP_characterPawn.curCharacter` (`self.PlayerRef`)))
  (`KismetSystemLibrary.PrintString` "Confirm Update PPS" true true (struct :`G` 1.0 :`B` 0.339962 :`A` 1.0)))

(event `ResetDefaultPPS`
  (bind _playerref (`self.PlayerRef`))
  (`KismetMaterialLibrary.SetScalarParameterValue` "/Game/MPC_PPS.MPC_PPS" "CelShadingDesatuation") ; Desaturation 0
  (`self.GrayscaleToColorful` false)
  (`self.TurnOffUnderWater`)
  (`self.EnableCelShading`)
  (`/Game/Main/Blueprints/Actors/BP_characterPawn.DpFPPSDestroy` _playerref)
  (set `Widget.Visibility` "Hidden" (`/Game/Main/Blueprints/Actors/BP_characterPawn.BPWSleepy` _playerref)))

(event `TurnOnVignette`
  (if (not (`self.IsVignetteOn`))
    (bind (_direction _radius) (`Timeline|VignetteRadius` :!via `PlayFromStart`)
      (:`Update`
        (`KismetMaterialLibrary.SetScalarParameterValue` "/Game/MPC_PPS.MPC_PPS" "CenterVignetteRadius" _radius))
      (:`Finished`
        (set `self.IsVignetteOn` true)))))

(event `TurnOffVignette`
  (if (`self.IsVignetteOn`)
    (bind (_direction _radius) (`Timeline|Timeline_1` :!via `ReverseFromEnd`)
      (:`Update`
        (`KismetMaterialLibrary.SetScalarParameterValue` "/Game/MPC_PPS.MPC_PPS" "CenterVignetteRadius" _radius))
      (:`Finished`
        (set `self.IsVignetteOn` false)))))

(fn `UserConstructionScript`)