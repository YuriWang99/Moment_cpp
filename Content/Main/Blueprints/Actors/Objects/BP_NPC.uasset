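; BP_NPC is an NPC actor blueprint that tracks a status, mood sounds and confirmation by other NPCs.
; It resets its status on begin play.
; PlayMoodSound picks a happy, sad or angry list from a mood SFX library, plays a random entry at the actor's location and stores the spawned audio handle.
; Confirmation events set or clear a second-layer confirmed flag and its indicator reference.
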(event `self.ReceiveBeginPlay`
  (`parent.ReceiveBeginPlay`)
  (set `self.CurStatus` "NewEnumerator0"))

(event `PlayMoodSound`
  (params (Mood :type "/Game/Main/Blueprints/Enum/E_Moods Enum" :default "NewEnumerator4"))
  (bind (_happysounds _sadsounds _angrysounds) (break `/Game/Main/Blueprints/Structures/S_NPCMoodSFX` (`self.MoodSFXLibrary`)))
  (switch `/Game/Main/Blueprints/Enum/E_Moods` Mood
    (:`NewEnumerator0`
      (`self.GetRandomSoundFromList` _happysounds))
    (:`NewEnumerator1`
      (`self.GetRandomSoundFromList` _sadsounds))
    (:`NewEnumerator2`
      (`self.GetRandomSoundFromList` _angrysounds))))

(event `GetRandomSoundFromList`
  (params (SoundArray :type "Array of SoundCue Object Reference"))
  (bind _returnvalue (`KismetArrayLibrary.Array_Length` SoundArray))
  (if (> _returnvalue 0)
    (bind _returnvalue_2 (`GameplayStatics.SpawnSoundAtLocation` (`|GetArrayItem` SoundArray (`KismetMathLibrary.RandomIntegerInRange` 0 (- _returnvalue 1))) (`self.K2_GetActorLocation`) (struct) 1.0 1.0 0.0 null null))
    (set `self.MoodSFXHandler` _returnvalue_2)))

(event `beConfirmedByNPC`
  (params (inputConfirmIndicator :type "/Game/Main/Blueprints/Actors/Objects/BP_NPC Object Reference"))
  ;[1 0.5652 0.09032] be confirmed by other NPC
  (set `self.isConfirmed_Layer2` true)
  (set `self.ConfirmIndicator` inputConfirmIndicator))

(event `ResetBeConfirmedState`
  ;[1 0.5652 0.09032] be confirmed by other NPC
  (set `self.isConfirmed_Layer2` false)
  (set `self.ConfirmIndicator` null))

(fn `UserConstructionScript`
  (`parent.UserConstructionScript`))