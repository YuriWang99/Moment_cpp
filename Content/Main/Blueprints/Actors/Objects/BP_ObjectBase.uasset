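; Base actor for interactable objects, NPCs included, that reveals the current NPC's thought about it as animated 3D text.
; ObjectInteract picks the mood-matched NPC thought or the default from that NPC's interaction maps, then triggers sparkle, sound and subtitles.
; TextShow copies a placed reference text's content and transform, applying the character's font and materials.
; Timelines drive per-character scale and location reveals, and exiting reverses the animation before re-enabling interaction.
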(event `self.ReceiveBeginPlay`
  (bind _text3d (`self.Text3D`))
  (bind _3dtextinworld (`self.3DTextInWorld`))
  (`SceneComponent.SetVisibility` _text3d false false)
  (`SceneComponent.K2_SetWorldRotation` :`self` _text3d)
  (`/Engine/EditorBlueprintResources/StandardMacros.IsValid` _3dtextinworld
    (:`Is Valid`
      (`SceneComponent.SetVisibility` (`self.GetComponentByClass` _3dtextinworld "/Script/Text3D.Text3DComponent") false false))))

(event `self.ReceiveTick`
  (params (DeltaSeconds :type "Float (single-precision)"))
  (`self.PlayerRef`
    (:`then`)
    (:`else`
      (bind _outactors (`GameplayStatics.GetAllActorsOfClass` "/Game/Main/Blueprints/Actors/BP_characterPawn.BP_characterPawn_C"))
      (set `self.PlayerRef` (`|GetArrayItem` _outactors)))))

(event `ObjectInteract`
  (params (`Current NPC` :type "/Game/Main/Blueprints/Actors/Objects/BP_NPC Object Reference"))
  (bind _playerref (`self.PlayerRef`))
  (bind (_value _returnvalue) (`BlueprintMapLibrary.Map_Find` (`/Game/Main/Blueprints/Actors/Objects/BP_NPC.CorrectNPCInteractionInfo` `Current NPC`) self))
  (bind (_value_2 _returnvalue_2) (`BlueprintMapLibrary.Map_Find` (`/Game/Main/Blueprints/Actors/Objects/BP_NPC.ObjInteractionInfo` `Current NPC`) self))
  (`|ExecutionSequence`
    (:`then_0`
      (if _returnvalue
        (bind _asbp_npc (cast `/Game/Main/Blueprints/Actors/Objects/BP_NPC` self)
          (:`then`
            (if (`|EnumEquality` (`/Game/Main/Blueprints/Actors/Objects/BP_NPC.CurMood` _asbp_npc) (`.Mood_11_3219A06D440F8CE8B3A9A181E9777B10` (break `/Game/Main/Blueprints/Structures/S_InteractionInfo` _value)))
              (bind (_output _textref _new_info) (`self.GetThoughtFromInteraction` _value))
              (`self.TextShow` _output _textref)
              (`NiagaraFunctionLibrary.SpawnSystemAtLocation` "/Game/Main/NarrativeTest/Demo/NS_Sparkle.NS_Sparkle" (`SceneComponent.K2_GetComponentLocation` (`self.Text3D`)) :!label _label)
              (`self.PlayInteractionSound`)
              (else
                (if _returnvalue_2 :!label _label_2
                  (bind (_output_2 _textref_2 _new_info_2) (`self.GetThoughtFromInteraction` _value_2))
                  (`self.TextShow` _output_2 _textref_2)
                  (goto _label)
                  (else
                    (`KismetSystemLibrary.PrintString` "Obi Interaction Not Found" true true (struct :`R` 1.0 :`G` 0.057555 :`A` 1.0))
                    (set `/Game/Main/Blueprints/Actors/BP_characterPawn.CanInteract` true (`self.PlayerRef`)))))))
          (:`CastFailed`
            (goto _label_2)))
        (else
          (goto _label_2))))
    (:`then_1`
      ;[1 0.5521 0.9076] Show Subtitle
      (bind _hittedobj (`/Game/Main/Blueprints/Actors/BP_characterPawn.HittedObj` (`self.PlayerRef`))
        (:`then`
          (bind (_value_3 _returnvalue_3) (`BlueprintMapLibrary.Map_Find` (`/Game/Main/Blueprints/Actors/Objects/BP_NPC.ObjInteractionInfo` (`/Game/Main/Blueprints/Actors/BP_characterPawn.curCharacter` (`self.PlayerRef`))) _hittedobj))
          (if _returnvalue_3
            ;[1 0.6226 0.1707] First Time Interactiong
            (if (`/Game/Main/Blueprints/Actors/BP_characterPawn.IsFirstTimeInteraction` _playerref)
              (bind ((`TargetObjSFX_30_49D5A7E4451C3FC7CF92D3A133799508` _targetobjsfx) (`Description_29_E87EEDC544924200C50059A89D8ED20E` _description)) (break `/Game/Main/Blueprints/Structures/S_InteractionInfo` _value_3))
              (`/Game/Main/NarrativeTest/Demo/BPW_Subtitle.Murmur` (`/Game/Main/Blueprints/Actors/BP_characterPawn.SubtitleUI` _playerref) (`/Game/Main/Blueprints/Actors/BP_characterPawn.InteractionIntro` _playerref) _description null)
              (`KismetSystemLibrary.PrintString` "First time interaction" true true (struct :`G` 1.0 :`B` 0.615812 :`A` 1.0) 4.0)
              (set `/Game/Main/Blueprints/Actors/BP_characterPawn.IsFirstTimeInteraction` false _playerref)
              (else
                (`/Game/Main/NarrativeTest/Demo/BPW_Subtitle.ShowSubtitle` (`/Game/Main/Blueprints/Actors/BP_characterPawn.SubtitleUI` (`self.PlayerRef`)) _description _hittedobj) ; Only show when the content is not empty
              ))))
        (:`else`)))))

(event `ObjectExitInteract`
  (if (`self.IsReadingText`)
    (`self.TextHide`)
    (`KismetSystemLibrary.Delay` 0.5)
    (set `/Game/Main/Blueprints/Actors/BP_characterPawn.CanInteract` true (`self.PlayerRef`))))

(event `TextShow`
  (params (TextToDisplay :type Text) (TextReference :type "/Game/Main/Blueprints/Text/BP_3DTextWorldSpace Object Reference"))
  (bind _text3dcharactertransform (`self.Text3DCharacterTransform`))
  (bind _text3d (`self.Text3D`))
  (bind _text_ref (`self.Text Ref`))
  (bind _text3d_2 (`self.Text3D`))
  (bind _text3d_3 (`self.Text3D`))
  (bind _rootcomponent (`Actor.RootComponent` _text_ref))
  (bind _curcharacter (`/Game/Main/Blueprints/Actors/BP_characterPawn.curCharacter` (`self.PlayerRef`)))
  (bind _npcfont (`/Game/Main/Blueprints/Actors/Objects/BP_NPC.NPCFont` _curcharacter))
  (set `self.Text Ref` TextReference)
  (set `self.IsReadingText` true)
  (`KismetSystemLibrary.PrintString` "TextShow" true true (struct :`R` 0.513839 :`B` 1.0 :`A` 1.0))
  (`/Engine/EditorBlueprintResources/StandardMacros.IsValid` (`self.Text Ref`)
    (:`Is Valid`
      (`SceneComponent.K2_SetWorldLocation` _text3d_2 (`SceneComponent.K2_GetComponentLocation` (`/Game/Main/Blueprints/Text/BP_3DTextWorldSpace.Text3D` _text_ref)) false false)
      (`SceneComponent.SetWorldScale3D` _text3d_2 (`SceneComponent.K2_GetComponentScale` _rootcomponent))
      (`SceneComponent.K2_SetWorldRotation` _text3d_2 (`SceneComponent.K2_GetComponentRotation` _rootcomponent) false false)
      ;[0.1017 0.06779 0.2802] Customize Thought font appearance
      (`/Engine/EditorBlueprintResources/StandardMacros.IsValid` _npcfont
        (:`Is Valid`
          (`Text3DComponent.SetFont` _text3d_3 _npcfont)
          (`self.Set3DTextMaterial` _text3d_3 (`/Game/Main/Blueprints/Actors/Objects/BP_NPC.NPCFontFront` _curcharacter) (`/Game/Main/Blueprints/Actors/Objects/BP_NPC.NPCFontBevel` _curcharacter) (`/Game/Main/Blueprints/Actors/Objects/BP_NPC.NPCFontExtrude` _curcharacter)))
        (:`Is Not Valid`
          _)))
    (:`Is Not Valid`
      (`/Game/Main/NarrativeTest/Demo/BP_FunctionLibrary_Aris.3DTextFacingCam` (`self.Text3D`))
      (`KismetSystemLibrary.PrintString` "No Text Ref" true true (struct :`R` 1.0 :`B` 0.040325 :`A` 1.0))))
  ;[0.5998 0.3604 0.8542] Has Separated 3D Text OR Not
  (`SceneComponent.SetVisibility` _text3d true false)
  (`Text3DComponent.SetText` _text3d (`Text3DComponent.Text` (`/Game/Main/Blueprints/Text/BP_3DTextWorldSpace.Text3D` TextReference)))
  (bind (_direction _scaleprogress _locationprogress) (`Timeline|Timeline` :!via `PlayFromStart`)
    (:`Update`
      (`Text3DCharacterTransform.SetScaleProgress` _text3dcharactertransform _scaleprogress)
      (`Text3DCharacterTransform.SetLocationProgress` _text3dcharactertransform _locationprogress))))

(event `TextHide`
  (bind _text3dcharactertransform (`self.Text3DCharacterTransform`))
  (set `self.IsReadingText` false)
  (`KismetSystemLibrary.PrintString` "TextHide" true true (struct :`R` 0.513839 :`B` 1.0 :`A` 1.0))
  ;[0.5998 0.3604 0.8542] Has Separated 3D Text OR Not
  (bind (_direction _scaleprogress _locationprogress) (`Timeline|Timeline_1` :!via `ReverseFromEnd`)
    (:`Update`
      (`Text3DCharacterTransform.SetScaleProgress` _text3dcharactertransform _scaleprogress)
      (`Text3DCharacterTransform.SetLocationProgress` _text3dcharactertransform _locationprogress))))

(event `PlayInteractionSound`
  (bind _playerref (`self.PlayerRef`)
    (:`then`
      (bind _wwisemanager (`/Game/Main/Blueprints/Actors/BP_characterPawn.WWiseManager` _playerref)
        (:`then`
          (`/Game/Main/Blueprints/BP_WwiseManager.SObjectInteract` _wwisemanager))
        (:`else`)))
    (:`else`)))

(fn `GetThoughtFromInteraction`
  (params (StructRef :type "/Game/Main/Blueprints/Structures/S_InteractionInfo Structure (by ref)"))
  (returns (Output :type Text) (TextRef :type "/Game/Main/Blueprints/Text/BP_3DTextWorldSpace Object Reference") (`New Info` :type "/Game/Main/Blueprints/Structures/S_InteractionInfo Structure"))
  (locals (ThoughtIndex :type Integer))
  (bind (_mood _npcthoughts _targetobjsfx _3dtext) (break `/Game/Main/Blueprints/Structures/S_InteractionInfo` StructRef))
  ;[0.1302 0.1302 0.1302] Get the thought text
  (bind _output (`/Game/Main/NarrativeTest/Demo/BP_FunctionLibrary_Aris.ReformatTextWithNewLine` (`Text3DComponent.Text` (`/Game/Main/Blueprints/Text/BP_3DTextWorldSpace.Text3D` _3dtext))))
  (return _output _3dtext))

(fn `Set3DTextMaterial`
  (params (Text3D :type "Text3DComponent Object Reference") (Front :type "MaterialInstance Object Reference") (Bevelm :type "MaterialInstance Object Reference") (Extrude :type "MaterialInstance Object Reference"))
  (`Text3DComponent.SetFrontMaterial` Text3D Front)
  (`Text3DComponent.SetBevelMaterial` Text3D Bevelm)
  (`Text3DComponent.SetExtrudeMaterial` Text3D Extrude)
  (`Text3DComponent.SetBackMaterial` Text3D Front)
  (return))

(fn `UpdateInteraction`
  (params (InteractionInfoMap :type "Map of /Game/Main/Blueprints/Actors/Objects/BP_ObjectBase Object Reference to /Game/Main/Blueprints/Structures/S_InteractionInfo Structure (by ref)") (KeyNPC :type "/Game/Main/Blueprints/Actors/Objects/BP_ObjectBase Object Reference (by ref)") (UpdatedValue :type "/Game/Main/Blueprints/Structures/S_InteractionInfo Structure (by ref)"))
  ;[0.03854 0.03854 0.03854] Update the Info structure
  (`BlueprintMapLibrary.Map_Remove` InteractionInfoMap KeyNPC)
  (`BlueprintMapLibrary.Map_Add` InteractionInfoMap KeyNPC UpdatedValue))

(fn `UserConstructionScript`)