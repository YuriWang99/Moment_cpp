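; Interactable world object that shows a 3D text description, hidden at BeginPlay.
; Interact sets and reveals the text with a show sequence and sparkle Niagara effect; ExitInteract plays a hide sequence, then hides it after a short delay.
; Tick continuously rotates the text based on the player's position.
; ChangeText swaps in a second front material and a phase-indexed description, then replays the show sequence.
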(event `self.ReceiveBeginPlay`
  (`self.Close3Dtest`)
  (set `self.DescriptionPhase` 0))

(event `Close3Dtest`
  (bind _text3d (`self.Text3D`))
  (`SceneComponent.SetVisibility` _text3d false false)
  (`SceneComponent.K2_SetWorldRotation` :`self` _text3d))

(event `Show3Dtest`
  (params (Actor :type "Vector Structure"))
  (bind _text3d (`self.Text3D`))
  (bind (_returnvalue_roll _returnvalue_pitch _returnvalue_yaw) (`KismetMathLibrary.BreakRotator` (`KismetMathLibrary.FindLookAtRotation` (`SceneComponent.K2_GetComponentLocation` _text3d) Actor)))
  (`SceneComponent.SetVisibility` _text3d true false)
  (`SceneComponent.K2_SetWorldRotation` _text3d (`KismetMathLibrary.MakeRotator` _returnvalue_roll (+ _returnvalue_pitch -90.0) (+ _returnvalue_yaw -180.0)) false false))

(event `self.ReceiveTick`
  (params (DeltaSeconds :type "Float (single-precision)"))
  ;[0.04271 0.04271 0.04271] Rotate 3D Text
  (`SceneComponent.K2_SetWorldRotation` (`self.Text3D`) (`KismetMathLibrary.FindLookAtRotation` (`self.K2_GetActorLocation` (`GameplayStatics.GetPlayerCharacter` 0)) (`SceneComponent.K2_GetComponentLocation` (`self.Text3D`))) false false))

(event `/Game/Main/NarrativeTest/AdvancedDialog/Interfaces/BPI_Interact.Interact`
  (bind _text3d (`self.Text3D`))
  (`Text3DComponent.SetText` _text3d (`KismetTextLibrary.Conv_StringToText` (`self.Description`)))
  (`SceneComponent.SetVisibility` _text3d true false)
  (`self.TextShow`)
  (`NiagaraFunctionLibrary.SpawnSystemAtLocation` "/Game/Main/NarrativeTest/Demo/NS_Sparkle.NS_Sparkle" (`SceneComponent.K2_GetComponentLocation` _text3d)))

(event `/Game/Main/NarrativeTest/AdvancedDialog/Interfaces/BPI_Interact.ExitInteract`
  (`self.TextHide`)
  (`KismetSystemLibrary.Delay` 0.5)
  (`SceneComponent.SetVisibility` (`self.Text3D`) false false))

(event `TextShow`
  (`ActorSequenceComponent.PlaySequence` (`self.ShowTextSequence`)))

(event `TextHide`
  (`ActorSequenceComponent.PlaySequence` (`self.HideTextSequence1`)))

(event `ChangeText`
  (params (Phase :type Integer))
  (bind _text3d (`self.Text3D`))
  (`Text3DComponent.SetFrontMaterial` _text3d (`self.SecondMaterial`))
  (`Text3DComponent.SetText` _text3d (`KismetTextLibrary.Conv_StringToText` (`|GetArrayItem` (`self.ChangedDescriptions`) Phase)))
  (`self.TextShow`))

(fn `UserConstructionScript`)