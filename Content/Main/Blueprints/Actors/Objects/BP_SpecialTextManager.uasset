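; Manager actor that shows special pop-up text tied to a particular NPC.
; On BeginPlay it binds to the player pawn's finish-switch-view event.
; ShowCharacterSpecialText checks the NPC's name enum and, on a single match, fires a one-time "Boring" PopUp on the referenced BoringSpecialText actor.
; ClearSpecialText hides that actor by scaling it to zero.
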(event `self.ReceiveBeginPlay`
  (bind _asbp_character_pawn (cast `/Game/Main/Blueprints/Actors/BP_characterPawn` (`GameplayStatics.GetPlayerCharacter` 0)))
  (bind _output_get (set `self.PlayerRef` _asbp_character_pawn))
  (add `/Game/Main/Blueprints/Actors/BP_characterPawn.OnFinishSwitchView` _output_get (`|CreateDelegate` :!event `ShowCharacterSpecialText`)))

(event `ShowCharacterSpecialText`
  (params (NewNPC :type "/Game/Main/Blueprints/Actors/Objects/BP_NPC Object Reference"))
  (if (`|EnumEquality` (`/Game/Main/Blueprints/Actors/Objects/BP_NPC.name_NPC` NewNPC) "NewEnumerator5")
    (`/Engine/EditorBlueprintResources/StandardMacros.DoOnce` false
      (:`Completed`
        (bind _boringspecialtext (`self.BoringSpecialText`)
          (:`then`
            (`/Game/Main/Blueprints/Text/BP_3DTextWorldSpace.PopUp` _boringspecialtext "Boring"))
          (:`else`))))))

(event `ClearSpecialText`
  (`self.SetActorScale3D` (`self.BoringSpecialText`) (0.0 0.0 0.0)))

(fn `UserConstructionScript`)