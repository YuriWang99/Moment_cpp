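; BP_oldNPC is an NPC actor Blueprint whose only active logic plays mood-based voice or sound effects.
; The PlayMoodSound event switches on a Happy, Sad or Anger mood and picks a random sound from the matching set in MoodSFXLibrary.
; It spawns that sound at the actor's location and stores the resulting audio component in MoodSFXHandler.
; BeginPlay, overlap, Tick and the construction script add no behavior.
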(event `PlayMoodSound`
  (params (Mood :type "/Game/Main/Blueprints/Enum/E_Moods Enum" :default "NewEnumerator4"))
  (bind _returnvalue (`self.K2_GetActorLocation`))
  (bind (_happysounds _sadsounds _angrysounds) (break `/Game/Main/Blueprints/Structures/S_NPCMoodSFX` (`self.Mood SFX Library`)))
  (switch `/Game/Main/Blueprints/Enum/E_Moods` Mood
    (:`NewEnumerator0`
      (bind _sound (`self.Get Random Sound from Struct` _happysounds))
      (bind _returnvalue_2 (`GameplayStatics.SpawnSoundAtLocation` _sound _returnvalue (struct) 1.0 1.0 0.0 null null))
      (set `self.MoodSFXHandler` _returnvalue_2))
    (:`NewEnumerator1`
      (bind _sound_2 (`self.Get Random Sound from Struct` _sadsounds))
      (bind _returnvalue_3 (`GameplayStatics.SpawnSoundAtLocation` _sound_2 _returnvalue (struct) 1.0 1.0 0.0 null null))
      (set `self.MoodSFXHandler` _returnvalue_3))
    (:`NewEnumerator2`
      (bind _sound_3 (`self.Get Random Sound from Struct` _angrysounds))
      (bind _returnvalue_4 (`GameplayStatics.SpawnSoundAtLocation` _sound_3 _returnvalue (struct) 1.0 1.0 0.0 null null))
      (set `self.MoodSFXHandler` _returnvalue_4))))

(fn `UserConstructionScript`
  (`parent.UserConstructionScript`))