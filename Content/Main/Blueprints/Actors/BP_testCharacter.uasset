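; Player character for a cursor-driven inspection game with Man and Girl viewpoints, including debug keys.
; Tick traces under the cursor, driving crosshair UI, custom-depth stencil highlights and interact messages.
; Clicks toggle confirmed objects in GM_testLevel, which checks them when hover ends, or switch camera points once the Man phase finishes.
; Switching plays a Level Sequence forward or reversed, swaps character visibility and re-clamps view limits; timelines ease camera panning.
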(event `HandleOnWin`
  (bind _man (`self.Man`))
  (bind _girl (`self.Girl`))
  ;[1 1 1] Handle On Win
  (`KismetSystemLibrary.Delay` 3.0)
  (`|ExecutionSequence`
    (:`then_0`
      (`self.SetActorHiddenInGame` _man false)
      (`self.SetActorEnableCollision` false)
      (`PrimitiveComponent.SetCustomDepthStencilValue` (`self.GetComponentByClass` _man "/Script/Engine.StaticMeshComponent") 0))
    (:`then_1`
      (`self.SetActorHiddenInGame` _girl false)
      (`self.SetActorEnableCollision` false)
      (`PrimitiveComponent.SetCustomDepthStencilValue` (`self.GetComponentByClass` _girl "/Script/Engine.StaticMeshComponent") 0))))

(event `Key|Zero`
  (params (Key :type "Key Structure"))
  ;[1 1 1] Test zone
  (:`Pressed`
    (`/Game/Main/Blueprints/GameMode/GM_testLevel.CheckPhase` (`self.GM_ref`) 0)))

(event `self.ReceiveBeginPlay`
  (`|ExecutionSequence`
    (:`then_0`
      (`self.InitUI`)
      (bind _outactors (`GameplayStatics.GetAllActorsOfClassWithTag` "/Script/LevelSequence.LevelSequenceActor" "SwitchCamera"))
      (set `self.LevelSequence` (`|GetArrayItem` _outactors))
      (`self.InitCamera`))
    (:`then_1`
      (`self.InitGMref`)
      (bind _outactors_2 (`GameplayStatics.GetAllActorsOfClassWithTag` "/Game/Main/Blueprints/Actors/Character/BP_Girl.BP_Girl_C" "Girl"))
      (bind _output_get (set `self.Girl` (`|GetArrayItem` _outactors_2)))
      (`self.SetActorHiddenInGame` _output_get false)
      (bind _outactors_3 (`GameplayStatics.GetAllActorsOfClassWithTag` "/Game/Main/Blueprints/Actors/Character/BP_Man.BP_Man_C" "Man"))
      (bind _output_get_2 (set `self.Man` (`|GetArrayItem` _outactors_3)))
      (`self.SetActorHiddenInGame` _output_get_2 true)
      (`self.SetActorEnableCollision` _output_get_2 false))
    (:`then_2`
      (set `self.CanInteract` true))
    (:`then_3`
      ;[1 1 1] Handle On Win
      (add `/Game/Main/Blueprints/GameMode/GM_testLevel.OnWin` (`self.GM_ref`) (delegate `HandleOnWin`)))
    (:`then_4`
      (set `PlayerController.CurrentMouseCursor` "Default" (`GameplayStatics.GetPlayerController` 0))
      (set `self.curViewIndex_Data` (`self.ViewIndex_Data_Man`)))))

(event `Key|One`
  (params (Key :type "Key Structure"))
  ;[1 1 1] Test zone
  (:`Pressed`
    (`/Game/Main/Blueprints/GameMode/GM_testLevel.FinishCheck` (`self.GM_ref`) "WatchMenu" 0)
    (`KismetSystemLibrary.PrintString` "Checked")))

(event `Key|Five`
  (params (Key :type "Key Structure"))
  ;[1 1 1] Test zone
)

(event `InitCameraSpline`
  (bind _outactors (`GameplayStatics.GetAllActorsOfClassWithTag` "/Game/Main/Blueprints/Actors/Objects/BP_CameraSpline.BP_CameraSpline_C" "CameraSpline"))
  (set `self.CameraSpline` (`|GetArrayItem` _outactors))
  (bind _outactors_2 (`GameplayStatics.GetAllActorsOfClassWithTag` "/Script/CinematicCamera.CineCameraActor" "CameraActor"))
  (set `self.CameraActor` (`|GetArrayItem` _outactors_2)))

(event `InitUI`
  (bind _returnvalue (`GameplayStatics.GetPlayerController` 0))
  ;[0.4485 1 0.3662] Init UI
  (bind _returnvalue_2 (`|CreateWidget` "/Game/Main/Blueprints/UI/WB_FirstPerson.WB_FirstPerson_C" (`GameplayStatics.GetPlayerController` 0)))
  (bind _output_get (set `self.WB_FirstPerson` _returnvalue_2))
  (`UserWidget.AddToViewport` _output_get 0)
  (bind _returnvalue_3 (`|CreateWidget` "/Game/Main/Blueprints/UI/WB_CursorTest.WB_CursorTest_C" _returnvalue))
  (`UserWidget.AddToViewport` _returnvalue_3 0)
  (set `self.WB_CursorTestref` _returnvalue_3)
  (set `PlayerController.bShowMouseCursor` true _returnvalue))

(event `InitGMref`
  ;[0.1311 0.917 1] Init Game Mode ref
  (bind _asgm_test_level (cast `/Game/Main/Blueprints/GameMode/GM_testLevel` (`GameplayStatics.GetGameMode`)))
  (set `self.GM_ref` _asgm_test_level)
  (`KismetSystemLibrary.PrintString` "Init GM_ref success"))

(event `InputAxis|LookLeft/Right`
  (params (AxisValue :type "Float (single-precision)"))
  ;[1 0.9825 0.1913] Camera control
)

(event `InputAxis|LookUp/Down`
  (params (AxisValue :type "Float (single-precision)"))
  ;[1 0.9825 0.1913] Camera control
)

(event `CursorHit`
  (bind (_hitresult _returnvalue) (`PlayerController.GetHitResultUnderCursorByChannel` (`GameplayStatics.GetPlayerController` 0) "TraceTypeQuery3" false))
  (bind (_bblockinghit _binitialoverlap _time _distance _location _impactpoint _normal _impactnormal _physmat _hitactor) (`GameplayStatics.BreakHitResult` _hitresult))
  (if _returnvalue
    (`KismetSystemLibrary.PrintString` (`KismetSystemLibrary.GetDisplayName` _hitactor) true true (struct :`R` 1.0 :`G` 0.858135 :`A` 1.0))
    (`|ExecutionSequence`
      (:`then_0`
        (if (`self.ActorHasTag` _hitactor "CameraPoint")
          (set `self.newCameraPos` null)
          (if (`/Game/Main/Blueprints/GameMode/GM_testLevel.manPhaseFinished` (`self.GM_ref`))
            _)
          (elif (`self.ActorHasTag` _hitactor "Interactable")
            (bind _output_get (set `self.HittedObj` _hitactor))
            (if (`KismetArrayLibrary.Array_Contains` (`/Game/Main/Blueprints/GameMode/GM_testLevel.ConfirmedActors` (`self.GM_ref`)) _output_get)
              (`self.SetStencilValue` _output_get 2)
              (bind _wb_firstperson (`self.WB_FirstPerson`)
                (:`then`
                  (message `/Game/Main/Blueprints/Interface/I_UI.I_ShowHitConfirm` _wb_firstperson))
                (:`else`))
              (else
                (`self.SetStencilValue` _output_get 1)
                (bind _wb_firstperson_2 (`self.WB_FirstPerson`)
                  (:`then`
                    (message `/Game/Main/Blueprints/Interface/I_UI.I_ShowHitMarker` _wb_firstperson_2))
                  (:`else`)))))))
      (:`then_1`
        (if (`KismetSystemLibrary.DoesImplementInterface` _hitactor "/Game/Main/NarrativeTest/AdvancedDialog/Interfaces/BPI_Interact.BPI_Interact_C")
          (if (not (== (`self.HittedObj`) (`self.PreviousActor`)))
            (`KismetSystemLibrary.PrintString` "Interaction start" true true (struct :`R` 1.0 :`G` 0.251122 :`B` 0.16141 :`A` 1.0))
            (message `/Game/Main/NarrativeTest/AdvancedDialog/Interfaces/BPI_Interact.Interact` (`self.HittedObj`))))))
    (else
      (`self.SetStencilValue` (`self.HittedObj`))
      (`self.WB_FirstPerson`
        (:`then`
          (message `/Game/Main/NarrativeTest/AdvancedDialog/Interfaces/BPI_Interact.ExitInteract` (`self.HittedObj`))
          ;[1 1 1] FinishCheck
          (bind _hittedobj (`self.HittedObj`)
            (:`then`
              (bind _asbp_interactable_object (cast `/Game/Main/Blueprints/Actors/Objects/BP_interactableObject` _hittedobj))
              (bind _objname (`/Game/Main/Blueprints/Actors/Objects/BP_interactableObject.objName` _asbp_interactable_object))
              (`/Game/Main/Blueprints/GameMode/GM_testLevel.FinishCheck` (`self.GM_ref`) _objname (`self.playerView`))
              (`KismetSystemLibrary.PrintString` _objname)
              (set `self.HittedObj` null))
            (:`else`)))
        (:`else`)))))

(event `self.ReceiveTick`
  (params (DeltaSeconds :type "Float (single-precision)"))
  (bind (_hitresult _returnvalue) (`PlayerController.GetHitResultUnderCursorByChannel` (`GameplayStatics.GetPlayerController` 0) "TraceTypeQuery3" false))
  (bind _iscameramoving (`/Game/Main/Blueprints/UI/WB_CursorTest.isCameraMoving` (`self.WB_CursorTestref`)))
  (bind (_bblockinghit _binitialoverlap _time _distance _location _impactpoint _normal _impactnormal _physmat _hitactor) (`GameplayStatics.BreakHitResult` _hitresult))
  (`KismetSystemLibrary.PrintString` (`KismetStringLibrary.Conv_BoolToString` _iscameramoving) true true (struct :`R` 1.0 :`G` 0.014381 :`A` 1.0))
  (if (not _iscameramoving)
    (`|ExecutionSequence`
      (:`then_0`
        (set `self.PreviousActor` (`self.HittedObj`)))
      (:`then_1`
        (if _returnvalue
          (`|ExecutionSequence`
            (:`then_0`
              ;[1 1 1] ShowHitmarker
              (if (`|EnumInequality` "NewEnumerator1" (`self.CurCrosshairState`))
                _
                (elif (`self.ActorHasTag` _hitactor "CameraPoint")
                  (set `self.newCameraPos` _hitactor)
                  ;[1 1 1] if the camera in the same
                  (if (`/Game/Main/Blueprints/GameMode/GM_testLevel.manPhaseFinished` (`self.GM_ref`))
                    (bind _wb_firstperson (`self.WB_FirstPerson`)
                      (:`then`
                        (message `/Game/Main/Blueprints/Interface/I_UI.I_ShowCameraIcon` _wb_firstperson)
                        (set `self.CurCrosshairState` "NewEnumerator3")
                        (set `PlayerController.CurrentMouseCursor` "GrabHand" (`GameplayStatics.GetPlayerController` 0)))
                      (:`else`)))
                  (elif (`self.ActorHasTag` _hitactor "Interactable")
                    (bind _output_get (set `self.HittedObj` _hitactor))
                    (if (`KismetArrayLibrary.Array_Contains` (`/Game/Main/Blueprints/GameMode/GM_testLevel.ConfirmedActors` (`self.GM_ref`)) _output_get)
                      (`self.SetStencilValue` _output_get 2)
                      (bind _wb_firstperson_2 (`self.WB_FirstPerson`)
                        (:`then`
                          (message `/Game/Main/Blueprints/Interface/I_UI.I_ShowHitConfirm` _wb_firstperson_2)
                          (set `self.CurCrosshairState` "NewEnumerator2"))
                        (:`else`))
                      (else
                        (`self.SetStencilValue` _output_get 1)
                        (bind _wb_firstperson_3 (`self.WB_FirstPerson`)
                          (:`then`
                            (message `/Game/Main/Blueprints/Interface/I_UI.I_ShowHitMarker` _wb_firstperson_3)
                            (set `self.CurCrosshairState` "NewEnumerator0"))
                          (:`else`))))
                    (else
                      ;[1 1 1] Close Hitmarker
                      (if (`|EnumEquality` (`self.CurCrosshairState`) "NewEnumerator0") :!label _label
                        (`self.SetStencilValue` (`self.HittedObj`))
                        (bind _wb_firstperson_4 (`self.WB_FirstPerson` :!label _label_2)
                          (:`then`
                            (message `/Game/Main/Blueprints/Interface/I_UI.I_CloseHitMarker` _wb_firstperson_4)
                            (`KismetSystemLibrary.PrintString` "Close Hit" true true (struct :`R` 1.0 :`G` 0.067316 :`B` 0.382197 :`A` 1.0))
                            (message `/Game/Main/NarrativeTest/AdvancedDialog/Interfaces/BPI_Interact.ExitInteract` (`self.HittedObj`))
                            (set `self.CurCrosshairState` "NewEnumerator1" :!label _label_3)
                            (set `PlayerController.CurrentMouseCursor` "Default" (`GameplayStatics.GetPlayerController` 0))
                            ;[1 1 1] FinishCheck
                            (bind _hittedobj (`self.HittedObj`)
                              (:`then`
                                (bind _asbp_interactable_object (cast `/Game/Main/Blueprints/Actors/Objects/BP_interactableObject` _hittedobj))
                                (bind _objname (`/Game/Main/Blueprints/Actors/Objects/BP_interactableObject.objName` _asbp_interactable_object))
                                (`/Game/Main/Blueprints/GameMode/GM_testLevel.FinishCheck` (`self.GM_ref`) _objname (`self.playerView`))
                                (`KismetSystemLibrary.PrintString` _objname)
                                (set `self.HittedObj` null))
                              (:`else`)))
                          (:`else`))
                        (elif (`|EnumEquality` (`self.CurCrosshairState`) "NewEnumerator2")
                          (goto _label_2)
                          (elif (`|EnumEquality` (`self.CurCrosshairState`) "NewEnumerator3")
                            (bind _wb_firstperson_5 (`self.WB_FirstPerson`)
                              (:`then`
                                (message `/Game/Main/Blueprints/Interface/I_UI.I_CloseCameraIcon` _wb_firstperson_5)
                                (goto _label_3))
                              (:`else`))))))))))
            (:`then_1`
              ;[0.1935 0.1305 0.6052] Interact
              (if (`KismetSystemLibrary.DoesImplementInterface` _hitactor "/Game/Main/NarrativeTest/AdvancedDialog/Interfaces/BPI_Interact.BPI_Interact_C")
                (if (not (== (`self.HittedObj`) (`self.PreviousActor`)))
                  (`KismetSystemLibrary.PrintString` "Interaction start" true true (struct :`R` 1.0 :`G` 0.251122 :`B` 0.16141 :`A` 1.0))
                  (message `/Game/Main/NarrativeTest/AdvancedDialog/Interfaces/BPI_Interact.Interact` (`self.HittedObj`))))))
          (else
            (goto _label)))))))

(event `SetStencilValue`
  (params (Actor :type "Actor Object Reference") (StencilValue :type Integer))
  (bind _gm_ref (`self.GM_ref`))
  (`/Engine/EditorBlueprintResources/StandardMacros.IsValid` Actor
    (:`Is Valid`
      (if (`self.ActorHasTag` Actor "Character")
        (if (== (and (`/Game/Main/Blueprints/GameMode/GM_testLevel.manPhaseFinished` _gm_ref) (`/Game/Main/Blueprints/GameMode/GM_testLevel.girlPhaseFinished` _gm_ref)) true)
          (`PrimitiveComponent.SetCustomDepthStencilValue` (`|GetArrayItem` (`self.GetComponentsByTag` Actor "/Script/Engine.StaticMeshComponent" "Mesh")) StencilValue :!label _label_4))
        (else
          (goto _label_4))))))

(event `InputAction|Mouse_1`
  (params (Key :type "Key Structure"))
  (bind _gm_ref (`self.GM_ref`))
  (bind _hittedobj (`self.HittedObj`))
  (bind _hittedobj_2 (`self.HittedObj`))
  (:`Released`
    ;[1 1 1] Show Hit Confirm
    (if (`|EnumEquality` "NewEnumerator0" (`self.CurCrosshairState`))
      (bind _wb_firstperson (`self.WB_FirstPerson`)
        (:`then`
          (message `/Game/Main/Blueprints/Interface/I_UI.I_ShowHitConfirm` _wb_firstperson)
          (set `self.CurCrosshairState` "NewEnumerator2")
          (`self.SetStencilValue` _hittedobj_2 2)
          (`/Game/Main/Blueprints/GameMode/GM_testLevel.AddConfirmActors` _gm_ref _hittedobj_2))
        (:`else`))
      (else
        ;[1 1 1] Close Hit Confirm
        (if (`|EnumEquality` "NewEnumerator2" (`self.CurCrosshairState`))
          (bind _wb_firstperson_2 (`self.WB_FirstPerson`)
            (:`then`
              (message `/Game/Main/Blueprints/Interface/I_UI.I_CloseHitConfirm` _wb_firstperson_2)
              (set `self.CurCrosshairState` "NewEnumerator0")
              (`self.SetStencilValue` _hittedobj 1)
              (`/Game/Main/Blueprints/GameMode/GM_testLevel.RemoveConfrimActors` _gm_ref _hittedobj))
            (:`else`)))))))

(event `InputAction|Mouse_0`
  (params (Key :type "Key Structure"))
  (:`Released`
    (if (`|EnumEquality` "NewEnumerator0" (`self.CurCrosshairState`))
      _
      (elif (`|EnumEquality` "NewEnumerator2" (`self.CurCrosshairState`))
        _
        (elif (`|EnumEquality` "NewEnumerator3" (`self.CurCrosshairState`))
          (bind _wb_firstperson (`self.WB_FirstPerson`)
            (:`then`
              (`/Game/Main/Blueprints/Interface/I_UI.I_CloseCameraIcon` _wb_firstperson)
              (bind _newcamerapos (`self.newCameraPos`)
                (:`then`
                  (`self.SwithCameraPos` _newcamerapos)
                  (set `self.CurCrosshairState` "NewEnumerator1"))
                (:`else`)))
            (:`else`)))))))

(event `OnFinished_Event`
  (bind _girl (`self.Girl`))
  (bind _man (`self.Man`))
  (bind _girl_2 (`self.Girl`))
  (bind _man_2 (`self.Man`))
  (switch `int` (`/Game/Main/Blueprints/Actors/Objects/BP_CameraPoint.characterView` (stale `SwithCameraPos` _asbp_camera_point))
    (:`0`
      (`self.SetActorHiddenInGame` _girl false)
      (`self.SetActorEnableCollision` _girl true)
      (`self.SetActorHiddenInGame` _man true)
      (`self.SetActorEnableCollision` _man false))
    (:`1`
      (`self.SetActorHiddenInGame` _girl_2 true)
      (`self.SetActorEnableCollision` _girl_2 false)
      (`self.SetActorHiddenInGame` _man_2 false)
      (`self.SetActorEnableCollision` _man_2 true))))

(event `SwithCameraPos`
  (params (newActorPos :type "Actor Object Reference"))
  (bind _returnvalue (`GameplayStatics.GetPlayerCameraManager` 0))
  (bind _returnvalue_2 (`self.GetTransform` newActorPos))
  (bind (_returnvalue_roll _returnvalue_pitch _returnvalue_yaw) (`KismetMathLibrary.BreakRotator` (`self.K2_GetActorRotation` newActorPos)))
  (bind _levelsequence (`self.LevelSequence`))
  (bind _sequenceplayer (`LevelSequenceActor.SequencePlayer` _levelsequence))
  (`|ExecutionSequence`
    (:`then_0`
      (bind _asbp_camera_point (cast `/Game/Main/Blueprints/Actors/Objects/BP_CameraPoint` newActorPos))
      (`self.SetActorHiddenInGame` (`self.Girl`) false)
      (`self.SetActorHiddenInGame` (`self.Man`) false)
      (set `self.curViewIndex` "NewEnumerator0")
      (switch `int` (`/Game/Main/Blueprints/Actors/Objects/BP_CameraPoint.characterView` _asbp_camera_point)
        (:`0`
          (`MovieSceneSequencePlayer.PlayReverse` _sequenceplayer)
          (set `self.curViewIndex_Data` (`self.ViewIndex_Data_Man`)))
        (:`1`
          (`MovieSceneSequencePlayer.Play` _sequenceplayer)
          (set `self.curViewIndex_Data` (`self.ViewIndex_Data_Girl`))))
      (add `MovieSceneSequencePlayer.OnFinished` (`LevelSequenceActor.SequencePlayer` _levelsequence) (delegate `OnFinished_Event`)))
    (:`then_1`
      (`self.K2_SetActorLocationAndRotation` (`KismetMathLibrary.MakeVector` (.x (.location _returnvalue_2)) (.y (.location _returnvalue_2)) (+ (.z (.location _returnvalue_2)) 10.0)) (.rotation _returnvalue_2))
      (`Controller.SetControlRotation` (`GameplayStatics.GetPlayerController` 0) (.rotation _returnvalue_2))
      (set `PlayerCameraManager.ViewYawMax` (+ _returnvalue_yaw (`self.YawMax`)) _returnvalue)
      (set `PlayerCameraManager.ViewYawMin` (+ _returnvalue_yaw (`self.YawMin`)) _returnvalue)
      (set `PlayerCameraManager.ViewPitchMax` (`self.PitchMax`) _returnvalue)
      (set `PlayerCameraManager.ViewPitchMin` (`self.PitchMin`) _returnvalue))
    (:`then_3`
      (set `self.playerView` (`/Game/Main/Blueprints/Actors/Objects/BP_CameraPoint.characterView` _asbp_camera_point))
      (`self.CameraSwitched`))))

(event `Key|Three`
  (params (Key :type "Key Structure"))
  (:`Pressed`
    (`self.CameraSwitched`)))

(event `Key|Four`
  (params (Key :type "Key Structure")))

(event `InputAction|Mouse_0`
  (params (Key :type "Key Structure"))
  (bind (_hitresult _returnvalue) (`PlayerController.GetHitResultUnderCursorByChannel` (`GameplayStatics.GetPlayerController` 0) "TraceTypeQuery3" false))
  (:`Released`
    (if _returnvalue
      (`KismetSystemLibrary.PrintString` (`KismetSystemLibrary.GetDisplayName` (`.HitActor` (`GameplayStatics.BreakHitResult` _hitresult))) true true (struct :`R` 1.0 :`G` 0.858135 :`A` 1.0)))))

(event `Key|MiddleMouseButton`
  (params (Key :type "Key Structure"))
  (:`Released`
    (set `self.CameraState` "NewEnumerator0")))

(event `MoveCamera`
  (bind _returnvalue (`GameplayStatics.GetPlayerController` 0))
  (bind (_direction _newtrack_0) (`Timeline|Timeline` :!via `PlayFromStart`)
    (:`Update`
      (`Controller.SetControlRotation` _returnvalue (`KismetMathLibrary.RLerp` (`Controller.GetControlRotation` _returnvalue) (`BlueprintMapLibrary.Map_Find` (`self.curViewIndex_Data`) (`self.curViewIndex`)) _newtrack_0)))))

(event `MoveRight`
  (bind (_direction _newtrack_0) (`Timeline|T_MoveRight` :!via `PlayFromStart` :!label _label)
    (:`Update`
      (`self.AddControllerYawInput` _newtrack_0))))

(event `MoveUp`
  (bind (_direction _newtrack_0) (`Timeline|T_MoveUp` :!via `PlayFromStart` :!label _label_2)
    (:`Update`
      (`self.AddControllerPitchInput` (* _newtrack_0 -1.0)))))

(event `stopMoveRight`
  (`|ExecutionSequence`
    (:`then_0`
      (goto _label :!via `Stop`))
    (:`then_1`
      (bind (_direction _newtrack_0) (`Timeline|T_stopingCamera` :!via `PlayFromStart`)
        (:`Update`
          (`self.AddControllerYawInput` _newtrack_0))))))

(event `stopMoveUp`
  (`|ExecutionSequence`
    (:`then_0`
      (goto _label_2 :!via `Stop`))
    (:`then_1`
      (bind (_direction _newtrack_0) (`Timeline|T_stopMoveUp` :!via `PlayFromStart`)
        (:`Update`
          (`self.AddControllerPitchInput` (* _newtrack_0 -1.0)))))))

(event `MoveLeft`
  (bind (_direction _newtrack_0) (`Timeline|T_MoveLeft` :!via `PlayFromStart` :!label _label_3)
    (:`Update`
      (`self.AddControllerYawInput` (* _newtrack_0 -1.0)))))

(event `MoveDown`
  (bind (_direction _newtrack_0) (`Timeline|T_MoveDown` :!via `PlayFromStart` :!label _label_4)
    (:`Update`
      (`self.AddControllerPitchInput` _newtrack_0))))

(event `stopMoveLeft`
  (`|ExecutionSequence`
    (:`then_0`
      (goto _label_3 :!via `Stop`))
    (:`then_1`
      (bind (_direction _newtrack_0) (`Timeline|T_stopingCameraLeft` :!via `PlayFromStart`)
        (:`Update`
          (`self.AddControllerYawInput` (* _newtrack_0 -1.0)))))))

(event `stopMoveDown`
  (`|ExecutionSequence`
    (:`then_0`
      (goto _label_4 :!via `Stop`))
    (:`then_1`
      (bind (_direction _newtrack_0) (`Timeline|T_stopMoveDown` :!via `PlayFromStart`)
        (:`Update`
          (`self.AddControllerPitchInput` _newtrack_0))))))

(fn `InitCamera`
  (bind _returnvalue (`GameplayStatics.GetPlayerCameraManager` 0))
  (bind (_returnvalue_roll _returnvalue_pitch _returnvalue_yaw) (`KismetMathLibrary.BreakRotator` (`self.K2_GetActorRotation` self)))
  ;[0.4485 1 0.3662] Init Camera
  (set `PlayerCameraManager.ViewYawMax` (+ _returnvalue_yaw (`self.YawMax`)) _returnvalue)
  (set `PlayerCameraManager.ViewYawMin` (+ _returnvalue_yaw (`self.YawMin`)) _returnvalue)
  (set `PlayerCameraManager.ViewPitchMax` (`self.PitchMax`) _returnvalue)
  (set `PlayerCameraManager.ViewPitchMin` (`self.PitchMin`) _returnvalue))

(fn `UserConstructionScript`)