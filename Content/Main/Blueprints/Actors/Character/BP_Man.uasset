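; BP_Man is a character actor with two 3D text components that display final words.
; On BeginPlay it hides both texts and binds to the OnWin dispatcher of GM_testLevel.
; ShowFinalWords reveals the texts, and HideFinalWords hides them after a short delay.
; Camera-facing calls for the texts are present but unconnected, so they never run.
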(event `self.ReceiveBeginPlay`
  (`SceneComponent.SetVisibility` (`self.Text3D`) false false)
  (`SceneComponent.SetVisibility` (`self.Text3D1`) false false)
  (bind _asgm_test_level (cast `/Game/Main/Blueprints/GameMode/GM_testLevel` (`GameplayStatics.GetGameMode`)))
  (add `/Game/Main/Blueprints/GameMode/GM_testLevel.OnWin` _asgm_test_level (`|CreateDelegate` :!event `HideFinalWords`)))

(event `self.ReceiveTick`
  (params (DeltaSeconds :type "Float (single-precision)")))

(event `ShowFinalWords`
  (`SceneComponent.SetVisibility` (`self.Text3D`) true false)
  (`SceneComponent.SetVisibility` (`self.Text3D1`) true false))

(event `HideFinalWords`
  (`KismetSystemLibrary.Delay` 3.0)
  (`SceneComponent.SetVisibility` (`self.Text3D`) false false)
  (`SceneComponent.SetVisibility` (`self.Text3D1`) false false))

(fn `UserConstructionScript`)