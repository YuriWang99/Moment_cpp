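; Base game mode for levels won by setting every NPC to its target mood.
; On BeginPlay it caches the player pawn and game instance, reads the current level, and hands tagged BP_NPC actors to the pawn.
; The win check compares each NPC's mood against a name-keyed map, firing the win call if all match or printing a retry message.
; The NPC confirming-state update loops without changing anything.
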(event `self.ReceiveBeginPlay`
  (`self.getReferences`)
  (`self.Init_Level`))

(event `Init_Level`
  (bind _character_ref (`self.Character_ref`))
  ;[0 0.4849 1] Init Level
  (`|ExecutionSequence`
    (:`then_0`
      (set `self.curLevel` (`/Game/Main/Blueprints/GameInstance/GI_Player.CurLevel` (`self.GI_player_ref`))))
    (:`then_1`
      (bind _outactors (`GameplayStatics.GetAllActorsOfClassWithTag` "/Game/Main/Blueprints/Actors/Objects/BP_NPC.BP_NPC_C" "NPC"))
      (bind _output_get (set `self.characterList` _outactors))
      (set `/Game/Main/Blueprints/Actors/BP_characterPawn.characterList` _output_get _character_ref)
      (`/Game/Main/Blueprints/Actors/BP_characterPawn.Init_character` _character_ref))))

(event `getReferences`
  ;[0 0.4849 1] get references
  (`|ExecutionSequence`
    (:`then_0`
      (bind _asbp_character_pawn (cast `/Game/Main/Blueprints/Actors/BP_characterPawn` (`GameplayStatics.GetPlayerCharacter` 0)))
      (set `self.Character_ref` _asbp_character_pawn))
    (:`then_1`
      (bind _asgi_player (cast `/Game/Main/Blueprints/GameInstance/GI_Player` (`GameplayStatics.GetGameInstance`)))
      (set `self.GI_player_ref` _asgi_player))))

(event `checkWinCondition`
  (bind _characterlist (`self.characterList`))
  ;[1 0.7401 0.03929] Check Win Condition
  (`self.UpdateNPC_ConfirmingState`)
  (for _array_element _characterlist
    (bind (_value _returnvalue) (`BlueprintMapLibrary.Map_Find` (`self.OnWin_characterMood`) (`/Game/Main/Blueprints/Actors/Objects/BP_ObjectBase.ObjName` _array_element)))
    (if _returnvalue
      (if (`|EnumEquality` _value (`/Game/Main/Blueprints/Actors/Objects/BP_NPC.CurMood` _array_element))
        (`/Engine/EditorBlueprintResources/StandardMacros.IncrementInt` (`self.CorrectedMood`))
        (else
          (break)))
      (else
        (break))))
  (if (== (`KismetArrayLibrary.Array_Length` _characterlist) (`self.CorrectedMood`))
    (`self.GM_OnWin`)
    (else
      (`KismetSystemLibrary.PrintString` "Try again" true true (struct :`R` 1.0 :`B` 0.014227 :`A` 1.0))
      (set `self.CorrectedMood` 0))))

(event `UpdateNPC_ConfirmingState`
  (for _array_element (`self.characterList`)
    (if (`/Game/Main/Blueprints/Actors/Objects/BP_NPC.isConfirmed_Layer2` _array_element)
      _)))

(fn `UserConstructionScript`)