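; Game mode for a two-level puzzle game that creates the HUD and initializes the level chosen by the game instance's CurLevel.
; Level 1 tracks per-view phase completion and wins when Man and Girl are both confirmed, triggering a Niagara effect and end sequence.
; Level 2 checks confirmed view/object pairs against an answer list, with a separate NPC mood check.
; Confirmation lists are capped, evicting the oldest pick and clearing its stencil highlight.
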(event `Level1_init`
  ;[1 1 1] Level1 Init
  (bind _outactors (`GameplayStatics.GetAllActorsOfClassWithTag` "/Script/LevelSequence.LevelSequenceActor" "EndSequence"))
  (set `self.EndSequence` (`|GetArrayItem` _outactors)))

(event `self.ReceiveBeginPlay`
  (`|ExecutionSequence`
    (:`then_0`
      (bind _asgi_player (cast `/Game/Main/Blueprints/GameInstance/GI_Player` (`GameplayStatics.GetGameInstance`)))
      (set `self.GI_player_ref` _asgi_player))
    (:`then_1`
      (bind _asbp_test_character (cast `/Game/Main/Blueprints/Actors/BP_testCharacter` (`GameplayStatics.GetPlayerCharacter` 0)))
      (set `self.PlayerRef` _asbp_test_character))
    (:`then_2`
      ;[1 0.3698 0.412] Narrative HUD Setup
      (bind _returnvalue (`|CreateWidget` "/Game/Main/NarrativeTest/AdvancedDialog/UserInterface/BPW_HUD.BPW_HUD_C"))
      (bind _output_get (set `self.HUD` _returnvalue))
      (`UserWidget.AddToViewport` _output_get 0))
    (:`then_3`
      (bind _output_get_2 (set `self.CurLevel` (`/Game/Main/Blueprints/GameInstance/GI_Player.CurLevel` (`self.GI_player_ref`))))
      (switch `int` _output_get_2
        (:`0`
          (`self.Level1_init`))
        (:`1`
          (`self.Level2 Init`))))))

(event `Level2 Init`
  ;[0 0.4849 1] Level 2 Init
  (bind _outactors (`GameplayStatics.GetAllActorsOfClassWithTag` "/Game/Main/Blueprints/Actors/Objects/NPC/BP_interactableNPC.BP_interactableNPC_C" "NPC"))
  (set `self.L2_CharacterList` _outactors))

(event `CheckWinCondition`
  ;[0 0.4849 1] Level2 win condition
  (for _array_element (`self.L2_CharacterList`)
    (bind (_value _returnvalue) (`BlueprintMapLibrary.Map_Find` (`self.L2_CharacterToMood`) (`/Game/Main/Blueprints/Actors/Objects/BP_interactableObject.objName` _array_element)))
    (if _returnvalue
      (if (not (`|EnumEquality` _value (`/Game/Main/Blueprints/Actors/Objects/NPC/BP_interactableNPC.curMood` _array_element)))
        (break))
      (else
        (break))))
  (`self.OnWin`))

(event `UpdateConfirmedActors`
  (bind _l2_s_confirmactors (`self.L2_S_ConfirmActors`))
  ;[1 1 1] Debug Cur Confirmed Actors
  (if (`KismetArrayLibrary.Array_IsNotEmpty` _l2_s_confirmactors)
    (for _array_element _l2_s_confirmactors
      (`KismetSystemLibrary.PrintString` (`KismetStringLibrary.Concat_StrStr` (`KismetStringLibrary.Conv_IntToString` (break `/Game/Main/Blueprints/Structures/S_Level2ConfirmActors` _array_element)) "/" (`.ObjName_9_7F33DC9E452DA708326BB1864D6BB3C6` (break `/Game/Main/Blueprints/Structures/S_Level2ConfirmActors` _array_element))) true true (struct :`G` 0.66 :`B` 1.0 :`A` 1.0) 1.0))
    (`KismetSystemLibrary.PrintString` "-------------------------------" true true (struct :`G` 0.66 :`B` 1.0 :`A` 1.0) 1.0)))

(event `SetConfirmedActor`
  (params (ActorLocation :type "Vector Structure"))
  (bind _confirmedactor (`self.ConfirmedActor`)
    (:`then`
      (cast `/Game/Main/Blueprints/Actors/Objects/BP_interactableObject` _confirmedactor))
    (:`else`)))

(event `UnsetConfirmActor`
  (bind _confirmedactor (`self.ConfirmedActor`)
    (:`then`
      (cast `/Game/Main/Blueprints/Actors/Objects/BP_interactableObject` _confirmedactor))
    (:`else`)))

(event `self.ReceiveTick`
  (params (DeltaSeconds :type "Float (single-precision)")))

(event `L2_AddConfirmActors`
  (params (PlayerView :type Integer) (ObjName :type String))
  (bind _l2_s_confirmactors (`self.L2_S_ConfirmActors`))
  (bind (_output_playerview _output_objname) (break `/Game/Main/Blueprints/Structures/S_Level2ConfirmActors` (`|GetArrayItem` _l2_s_confirmactors)))
  ;[0 0.4202 1] Level 2 Confirm
  (if (not (< (`KismetArrayLibrary.Array_Length` (`self.L2_S_ConfirmActors`)) 3))
    (bind _outactors (`GameplayStatics.GetAllActorsOfClass` "/Game/Main/Blueprints/Actors/Objects/BP_interactableObject.BP_interactableObject_C"))
    (for _array_element _outactors
      (if (`KismetStringLibrary.EqualEqual_StrStr` (`/Game/Main/Blueprints/Actors/Objects/BP_interactableObject.objName` _array_element) _output_objname)
        (`PrimitiveComponent.SetCustomDepthStencilValue` (`self.GetComponentByClass` _array_element "/Script/Engine.StaticMeshComponent") 0)
        (`KismetArrayLibrary.Array_Remove` _l2_s_confirmactors)
        (break))))
  (`KismetArrayLibrary.Array_AddUnique` (`self.L2_S_ConfirmActors`) (make `/Game/Main/Blueprints/Structures/S_Level2ConfirmActors` PlayerView ObjName))
  (`self.L2_CheckConfirmedActors`))

(event `L1_AddConfirmActors`
  (params (AddActor :type "Actor Object Reference"))
  ;[1 0.2416 0.9258] Level1 Check
  (if (not (< (`KismetArrayLibrary.Array_Length` (`self.L1_ConfirmedActors`)) 2))
    (`PrimitiveComponent.SetCustomDepthStencilValue` (`self.GetComponentByClass` (`|GetArrayItem` (`self.L1_ConfirmedActors`)) "/Script/Engine.StaticMeshComponent") 0)
    (`KismetArrayLibrary.Array_Remove` (`self.L1_ConfirmedActors`)))
  (`KismetArrayLibrary.Array_AddUnique` (`self.L1_ConfirmedActors`) AddActor)
  (bind _asbp_man (cast `/Game/Main/Blueprints/Actors/Character/BP_Man` AddActor)
    (:`then`
      (`/Game/Main/Blueprints/Actors/Character/BP_Man.ShowFinalWords` _asbp_man))
    (:`CastFailed`
      (bind _asbp_girl (cast `/Game/Main/Blueprints/Actors/Character/BP_Girl` AddActor)
        (:`then`
          (`/Game/Main/Blueprints/Actors/Character/BP_Girl.ShowFinalWords` _asbp_girl))
        (:`CastFailed`
          _))))
  (`self.L1_CheckConfirmActors`))

(event `L1_RemoveConfrimActors`
  (params (UnsetActor :type "Actor Object Reference"))
  ;[1 0.2416 0.9258] Level1 Check
  (`KismetArrayLibrary.Array_RemoveItem` (`self.L1_ConfirmedActors`) UnsetActor))

(event `L2_RemoveConfirmActors`
  (params (PlayerView :type Integer) (ObjName :type String))
  ;[0 0.4202 1] Level 2 Confirm
  (`KismetArrayLibrary.Array_RemoveItem` (`self.L2_S_ConfirmActors`) (make `/Game/Main/Blueprints/Structures/S_Level2ConfirmActors` PlayerView ObjName)))

(event `L1_CheckConfirmActors`
  (bind _l1_confirmedactors (`self.L1_ConfirmedActors`))
  (bind _playerref (`self.PlayerRef`))
  ;[1 0.2416 0.9258] Level1 Check
  (if (== (`KismetArrayLibrary.Array_Length` _l1_confirmedactors) 2)
    (if (and (`KismetArrayLibrary.Array_Contains` _l1_confirmedactors (`/Game/Main/Blueprints/Actors/BP_testCharacter.Man` _playerref)) (`KismetArrayLibrary.Array_Contains` _l1_confirmedactors (`/Game/Main/Blueprints/Actors/BP_testCharacter.Girl` _playerref)))
      (`self.OnWin`)
      (`NiagaraFunctionLibrary.SpawnSystemAtLocation` "/Game/Heart/NewNiagaraSystem.NewNiagaraSystem" (120.0 356.0 93.0) (struct) (1.0 1.0 1.0) false)
      (`KismetSystemLibrary.Delay` 3.0)
      (`MovieSceneSequencePlayer.Play` (`LevelSequenceActor.SequencePlayer` (`self.EndSequence`))))))

(event `L2_CheckConfirmedActors`
  (bind _l2_confirmlist (`self.L2_ConfirmList`))
  (bind _l2_s_confirmactors (`self.L2_S_ConfirmActors`))
  ;[0 0.4202 1] Level 2 Confirm
  (if (== (`KismetArrayLibrary.Array_Length` _l2_confirmlist) (`KismetArrayLibrary.Array_Length` _l2_s_confirmactors))
    (for _array_element _l2_s_confirmactors
      (if (not (`KismetArrayLibrary.Array_Contains` _l2_confirmlist _array_element))
        (break)))
    (`self.OnWin`)))

(event `L1_FinishCheck`
  (params (objName :type String) (playerView :type Integer))
  ;[1 0.2416 0.9258] Level1 Check
  (switch `int` playerView
    (:`Default`
      (`KismetSystemLibrary.PrintString` "invalid view" true true (struct :`R` 1.0 :`B` 0.051994 :`A` 1.0)))
    (:`0`
      (`BlueprintMapLibrary.Map_Add` (`self.Phase0_man`) objName true)
      (`self.CheckPhase` playerView :!label _label))
    (:`1`
      (`BlueprintMapLibrary.Map_Add` (`self.Phase1_woman`) objName true)
      (goto _label))))

(event `OpenLevel`
  ;[1 0.9825 0.1913] Open Level2
  (`/Engine/EditorBlueprintResources/StandardMacros.IncrementInt` (`/Game/Main/Blueprints/GameInstance/GI_Player.CurLevel` (`self.GI_player_ref`))
    (:`  `
      (`KismetSystemLibrary.ExecuteConsoleCommand` "servertravel /Game/Main/Levels/Level2_test" (`GameplayStatics.GetPlayerController` 0)))))

(fn `CheckPhase`
  (params (playerView :type Integer))
  (locals (Finished :type Boolean :default true))
  (switch `int` playerView
    (:`0`
      (bind _values (`BlueprintMapLibrary.Map_Values` (`self.Phase0_man`)))
      (for _array_element _values
        (if (not _array_element)
          (set `local.Finished` false)))
      (if (`local.Finished`)
        (`KismetSystemLibrary.PrintString` (`KismetStringLibrary.Concat_StrStr` (`KismetStringLibrary.Conv_IntToString` (`local.playerView`)) ": Phase finish") true true (struct :`R` 1.0 :`G` 0.208208 :`A` 1.0))
        (set `self.manPhaseFinished` true)
        (`self.onManPhaseFinish`)
        (else
          (`KismetSystemLibrary.PrintString` "Phase not finish" true true (struct :`R` 1.0 :`G` 0.208208 :`A` 1.0)))))
    (:`1`
      (bind _values_2 (`BlueprintMapLibrary.Map_Values` (`self.Phase1_woman`)))
      (for _array_element_2 _values_2
        (if (not _array_element_2)
          (set `local.Finished` false)))
      (if (`local.Finished`)
        (`KismetSystemLibrary.PrintString` (`KismetStringLibrary.Concat_StrStr` (`KismetStringLibrary.Conv_IntToString` (`local.playerView`)) ": Phase finish") true true (struct :`R` 1.0 :`G` 0.208208 :`A` 1.0))
        (set `self.girlPhaseFinished` true)
        (`self.onGirlPhaseFinish`)
        (else
          (`KismetSystemLibrary.PrintString` "Phase not finish" true true (struct :`R` 1.0 :`G` 0.208208 :`A` 1.0)))))))

(fn `UserConstructionScript`)